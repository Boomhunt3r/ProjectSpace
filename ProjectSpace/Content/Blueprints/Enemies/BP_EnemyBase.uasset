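; Base tower-defense enemy that walks toward a Destination, with Health, Shield and a health widget bound to it.
; Overlapping projectiles feed GetDamage and are destroyed; weapon type scales the damage, with heavy weapons favored against shields and MGs against bare health.
; Tick reissues the move while alive; at zero health, it removes itself from the "Tower_Ground" towers cached at BeginPlay, then destroys itself.
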(event `self.ReceiveBeginPlay`
  (bind _outactors (`GameplayStatics.GetAllActorsWithTag` "Tower_Ground"))
  (set `self.Towers` _outactors)
  (bind _asui_enemy_health (cast `/Game/Blueprints/Enemies/UI_Enemy_Health` (`WidgetComponent.GetUserWidgetObject` (`self.Widget`))))
  (`/Game/Blueprints/Enemies/UI_Enemy_Health.Unique Owner` _asui_enemy_health self))

(event `self.ReceiveActorBeginOverlap`
  (params (OtherActor :type "Actor Object Reference"))
  ;[1 1 1] Enemy hit logic
  (if (`self.ActorHasTag` OtherActor "Projectile")
    (bind _asbp_test_projectile (cast `/Game/Blueprints/BP_TestProjectile` OtherActor))
    (bind _output_get (set `self.Bullet` _asbp_test_projectile))
    (`self.GetDamage` (`KismetMathLibrary.Conv_IntToDouble` (`/Game/Blueprints/BP_TestProjectile.Damage` _output_get)) (`/Game/Blueprints/BP_TestProjectile.WeaponType` _output_get))
    (`self.K2_DestroyActor` _output_get)))

(event `self.ReceiveTick`
  (params (DeltaSeconds :type "Float (single-precision)"))
  (if (<= (`self.Health`) 0.0)
    (for _array_element (`self.Towers`)
      (bind _asbp_tower (cast `/Game/Blueprints/Tower/BP_Tower` _array_element))
      (`/Game/Blueprints/Tower/BP_Tower.RemoveFromArray` _asbp_tower self))
    (`self.K2_DestroyActor`)
    (else
      (`AIBlueprintHelperLibrary.SimpleMoveToActor` (`self.GetController`) (`self.Destination`)))))

(fn `GetDamage`
  (params (Damage :type "Float (double-precision)") (WeaponType :type "/Game/Enums/EWeaponType Enum" :default "NewEnumerator0"))
  (locals (`Weapon Type` :type "/Game/Enums/EWeaponType Enum") (IncomingDamge :type "Float (double-precision)"))
  (set `local.IncomingDamge` Damage)
  (set `local.Weapon Type` WeaponType)
  (if (> (`self.Shield`) 0.0)
    (switch `/Game/Enums/EWeaponType` (`local.Weapon Type`)
      (:`NewEnumerator0`
        (set `self.Shield` (- (`self.Shield`) (* (`local.IncomingDamge`) 1.0)))
        (set `self.Health` (- (`self.Health`) (* (`local.IncomingDamge`) 0.25))))
      (:`NewEnumerator1`
        (set `self.Shield` (- (`self.Shield`) (* (`local.IncomingDamge`) 0.25))))
      (:`NewEnumerator2`
        (set `self.Shield` (- (`self.Shield`) (* (`local.IncomingDamge`) 1.0)))
        (set `self.Health` (- (`self.Health`) (* (`local.IncomingDamge`) 0.25))))
      (:`NewEnumerator3`
        (set `self.Shield` (- (`self.Shield`) (* (`local.IncomingDamge`) 0.25)))))
    (elif (<= (`self.Shield`) 0.0)
      (switch `/Game/Enums/EWeaponType` (`local.Weapon Type`)
        (:`NewEnumerator0`
          (set `self.Health` (- (`self.Health`) (* (`local.IncomingDamge`) 0.8))))
        (:`NewEnumerator1`
          (set `self.Health` (- (`self.Health`) (* (`local.IncomingDamge`) 1.0))))
        (:`NewEnumerator2`
          (set `self.Health` (- (`self.Health`) (* (`local.IncomingDamge`) 0.8))))
        (:`NewEnumerator3`
          (set `self.Health` (- (`self.Health`) (* (`local.IncomingDamge`) 1.0))))))))

(fn `UserConstructionScript`)