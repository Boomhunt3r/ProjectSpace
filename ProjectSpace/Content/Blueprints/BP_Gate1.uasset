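; BP_Gate1 is a four-part gate that opens when actors enter its collision volume and closes when the last one leaves.
; An overlap counter and open flag gate two separate timelines that animate the Y scale of four locators.
; Opening sets world scale, while closing reverses the second timeline on relative scale and clears the flag during updates.
; The construction script applies GateMaterial to all four gate pieces.
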(event `self.Collision.OnComponentBeginOverlap`
  (params (OverlappedComponent :type "PrimitiveComponent Object Reference") (OtherActor :type "Actor Object Reference") (OtherComp :type "PrimitiveComponent Object Reference") (OtherBodyIndex :type Integer) (bFromSweep :type Boolean) (SweepResult :type "HitResult Structure (by ref)"))
  (`/Engine/EditorBlueprintResources/StandardMacros.IncrementInt` (`self.Actors in Overlap`)
    (:`  `
      (if (not (`self.Gate is open`))
        (set `self.Gate is open` true)
        (bind (_direction _scale_z) (`Timeline|scale Gate` :!via `PlayFromStart`)
          (:`Update`
            (`SceneComponent.SetWorldScale3D` (`self.Locator_01`) (`KismetMathLibrary.MakeVector` 1.0 _scale_z 1.0))
            (`SceneComponent.SetWorldScale3D` (`self.Locator_02`) (`KismetMathLibrary.MakeVector` 1.0 _scale_z 1.0))
            (`SceneComponent.SetWorldScale3D` (`self.Locator_03`) (`KismetMathLibrary.MakeVector` 1.0 _scale_z 1.0))
            (`SceneComponent.SetWorldScale3D` (`self.Locator_04`) (`KismetMathLibrary.MakeVector` 1.0 _scale_z 1.0))))))))

(event `self.Collision.OnComponentEndOverlap`
  (params (OverlappedComponent :type "PrimitiveComponent Object Reference") (OtherActor :type "Actor Object Reference") (OtherComp :type "PrimitiveComponent Object Reference") (OtherBodyIndex :type Integer))
  (`/Engine/EditorBlueprintResources/StandardMacros.DecrementInt` (`self.Actors in Overlap`)
    (:`  `
      (if (not (> (`self.Actors in Overlap`) 0))
        (bind (_direction _scale_z) (`Timeline|Timeline_0` :!via `ReverseFromEnd`)
          (:`Update`
            (`SceneComponent.SetRelativeScale3D` (`self.Locator_01`) (`KismetMathLibrary.MakeVector` 1.0 _scale_z 1.0))
            (`SceneComponent.SetRelativeScale3D` (`self.Locator_02`) (`KismetMathLibrary.MakeVector` 1.0 _scale_z 1.0))
            (`SceneComponent.SetRelativeScale3D` (`self.Locator_03`) (`KismetMathLibrary.MakeVector` 1.0 _scale_z 1.0))
            (`SceneComponent.SetRelativeScale3D` (`self.Locator_04`) (`KismetMathLibrary.MakeVector` 1.0 _scale_z 1.0))
            (set `self.Gate is open` false)))))))

(fn `UserConstructionScript`
  (`PrimitiveComponent.SetMaterial` (`self.Gate_01`) 0 (`self.Gate material`))
  (`PrimitiveComponent.SetMaterial` (`self.Gate_02`) 0 (`self.Gate material`))
  (`PrimitiveComponent.SetMaterial` (`self.Gate_03`) 0 (`self.Gate material`))
  (`PrimitiveComponent.SetMaterial` (`self.Gate_04`) 0 (`self.Gate material`)))