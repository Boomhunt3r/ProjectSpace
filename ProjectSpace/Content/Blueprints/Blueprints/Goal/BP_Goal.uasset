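; BP_Goal is the track-end goal that checks each cube's RGB values against a target color and tracks score.
; Cube arrival ends the round, stops turret tracking, starts the next, faster cube and calls SetColor for a new target, varied by game mutator.
; Mismatches stop the cube at a timeline-driven trapdoor.
; The success trigger increments score with faded audio; in Rush, the fail trigger decrements it and resets the trapdoor.
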(event `self.ReceiveBeginPlay`
  ;[1 1 1] Start Up
  (bind _outactors (`GameplayStatics.GetAllActorsOfClass` "/Game/Blueprints/Blueprints/Tower/BP_TowerBase.BP_TowerBase_C"))
  (set `self.Turrets` _outactors)
  (bind _returnvalue (`GameplayStatics.GetActorOfClass` "/Game/Blueprints/Blueprints/BP_Storage.BP_Storage_C"))
  (set `self.BP_Storage` _returnvalue)
  (bind _returnvalue_2 (`GameplayStatics.GetActorOfClass` "/Game/Blueprints/Blueprints/Cube/BP_CubeManager.BP_CubeManager_C"))
  (set `self.CubeManagerRef` _returnvalue_2)
  (bind _asbp_player (cast `/Game/Blueprints/Blueprints/Player/BP_Player` (`GameplayStatics.GetPlayerPawn` 0)))
  (set `self.PlayerRef` _asbp_player)
  (bind _returnvalue_3 (`GameplayStatics.GetActorOfClass` "/Game/Blueprints/Blueprints/Gamemode_Manager/BP_GameManager.BP_GameManager_C"))
  (set `self.GameManagerRef` _returnvalue_3)
  (bind _foundwidgets (`WidgetBlueprintLibrary.GetAllWidgetsOfClass` "/Game/UI/UI_ColorCode.UI_ColorCode_C" false))
  (set `self.ColorCode-Widget-Ref` (`|GetArrayItem` _foundwidgets)))

(event `self.Trapdoor_Stop.OnComponentBeginOverlap`
  (params (OverlappedComponent :type "PrimitiveComponent Object Reference") (OtherActor :type "Actor Object Reference") (OtherComp :type "PrimitiveComponent Object Reference") (OtherBodyIndex :type Integer) (bFromSweep :type Boolean) (SweepResult :type "HitResult Structure (by ref)"))
  ;[1 1 1] Trapdoor
  ;;[1 1 1] Stop Cube at Trapdoor
  (if (`self.ActorHasTag` OtherActor "Cube")
    (bind _asbp_cube (cast `/Game/Blueprints/Blueprints/Cube/BP_Cube` OtherActor))
    (if (`self.Wrong color`)
      (set `/Game/Blueprints/Blueprints/Cube/BP_Cube.Cube Movement Speed` 0.0 _asbp_cube)
      (`PrimitiveComponent.SetCollisionEnabled` (`self.hiddenBox`) "NoCollision"))))

(event `self.Entry.OnComponentBeginOverlap`
  (params (OverlappedComponent :type "PrimitiveComponent Object Reference") (OtherActor :type "Actor Object Reference") (OtherComp :type "PrimitiveComponent Object Reference") (OtherBodyIndex :type Integer) (bFromSweep :type Boolean) (SweepResult :type "HitResult Structure (by ref)"))
  (bind _bp_storage (`self.BP_Storage`))
  (bind _cubemanagerref (`self.CubeManagerRef`))
  (bind _ui_hud (`/Game/Blueprints/Blueprints/Player/BP_Player.UI_HUD` (`self.PlayerRef`)))
  ;[1 1 1] Cube has Reached Track End
  (if (`self.ActorHasTag` OtherActor "Cube")
    (bind _asbp_cube (cast `/Game/Blueprints/Blueprints/Cube/BP_Cube` OtherActor))
    (set `/Game/UI/UI_HUD.PressedFastForward` false _ui_hud)
    (set `/Game/UI/UI_HUD.Cube Ref` _asbp_cube _ui_hud)
    (for _array_element (`self.Turrets`)
      (set `/Game/Blueprints/Blueprints/Tower/BP_TowerBase.should follow Target` false _array_element))
    (set `/Game/Blueprints/Blueprints/BP_Storage.Round running` false _bp_storage)
    (`/Engine/EditorBlueprintResources/StandardMacros.IncrementFloat` (`self.Cubes passed`)
      (:`  `
        (`/Game/Blueprints/Blueprints/BP_Storage.Teleport_Board` _bp_storage)
        (`/Game/Blueprints/Blueprints/Cube/BP_CubeManager.Add Speed ` _cubemanagerref)
        (`/Game/Blueprints/Blueprints/Cube/BP_CubeManager.StartNextCube` _cubemanagerref)
        (`SceneComponent.SetVisibility` (`/Game/Blueprints/Blueprints/Cube/BP_Cube.Widget` _asbp_cube) false false)
        ;;[1 1 1] compare Color
        (`self.CompareColor` (`/Game/Blueprints/Blueprints/Cube/BP_Cube.Red` _asbp_cube) (`/Game/Blueprints/Blueprints/Cube/BP_Cube.Green` _asbp_cube) (`/Game/Blueprints/Blueprints/Cube/BP_Cube.Blue` _asbp_cube))
        ;;[1 1 1] Set new Target Color
        (`self.SetColor`)
        (`GameplayStatics.PlaySound2D` "/Game/StarterContent/Audio/Explosion01.Explosion01" 0.1 1.0 0.0 null null)
        (`/Game/UI/UI_ColorCode.Color has Changed/Play Animation` (`self.ColorCode-Widget-Ref`))))))

(event `self.Trapdoor_Trigger.OnComponentBeginOverlap`
  (params (OverlappedComponent :type "PrimitiveComponent Object Reference") (OtherActor :type "Actor Object Reference") (OtherComp :type "PrimitiveComponent Object Reference") (OtherBodyIndex :type Integer) (bFromSweep :type Boolean) (SweepResult :type "HitResult Structure (by ref)"))
  ;[1 1 1] Trapdoor
  (if (`self.Wrong color`)
    (bind (_direction _newtrack_2) (`Timeline|open Trapdoor` :!via `PlayFromStart` :!label _label)
      (:`Update`
        (`SceneComponent.K2_SetRelativeRotation` (`self.Trapdoor_01`) (`KismetMathLibrary.MakeRotator` 0.0 _newtrack_2 90.0) false false)
        (`SceneComponent.K2_SetRelativeRotation` (`self.Trapdoor_02`) (`KismetMathLibrary.MakeRotator` 0.0 _newtrack_2 -90.0) false false)))))

(event `self.C_FailCounter.OnComponentBeginOverlap`
  (params (OverlappedComponent :type "PrimitiveComponent Object Reference") (OtherActor :type "Actor Object Reference") (OtherComp :type "PrimitiveComponent Object Reference") (OtherBodyIndex :type Integer) (bFromSweep :type Boolean) (SweepResult :type "HitResult Structure (by ref)"))
  ;[1 1 1] Trapdoor
  ;;[1 1 1] Decrement Score and close Trapdoor (Rush only)
  (switch `/Game/Blueprints/Enums/EGameMode` (`/Game/Blueprints/Blueprints/Gamemode_Manager/BP_GameManager.GameMode` (`self.GameManagerRef`))
    (:`NewEnumerator2`
      (if (`self.ActorHasTag` OtherActor "Cube")
        (`/Engine/EditorBlueprintResources/StandardMacros.DecrementInt` (`self.Success Counter`)
          (:`  `
            (`PrimitiveComponent.SetCollisionEnabled` (`self.hiddenBox`) "QueryAndPhysics")
            (set `self.Wrong color` false)
            (goto _label :!via `ReverseFromEnd`)))))))

(event `self.C_SuccessCounter.OnComponentBeginOverlap`
  (params (OverlappedComponent :type "PrimitiveComponent Object Reference") (OtherActor :type "Actor Object Reference") (OtherComp :type "PrimitiveComponent Object Reference") (OtherBodyIndex :type Integer) (bFromSweep :type Boolean) (SweepResult :type "HitResult Structure (by ref)"))
  (bind _audio (`self.Audio`))
  ;[1 1 1] Success
  ;;[1 1 1] Count Success
  (if (`self.ActorHasTag` OtherActor "Cube")
    (`/Engine/EditorBlueprintResources/StandardMacros.IncrementInt` (`self.Success Counter`)
      (:`  `
        ;;[1 1 1] Succes Sound - muss mit nem richtigen Ton nochmal überarbeitet werden
        (`AudioComponent.SetVolumeMultiplier` _audio 1.0)
        (`AudioComponent.FadeIn` _audio 0.5 1.0 0.0 "Linear")
        (`KismetSystemLibrary.Delay` 0.5)
        (`AudioComponent.FadeOut` _audio 0.7 0.0 "Linear")
        (`KismetSystemLibrary.Delay` 1.0)
        (`AudioComponent.SetVolumeMultiplier` (`self.Audio`) 0.0)))))

(fn `CompareColor`
  (params (CubeRed :type Integer) (CubeGreen :type Integer) (CubeBlue :type Integer))
  (if (== CubeRed (`self.Red`))
    (if (== CubeGreen (`self.Green`))
      (if (not (== CubeBlue (`self.Blue`)))
        (set `self.Wrong color` true))
      (else
        (set `self.Wrong color` true)))
    (else
      (set `self.Wrong color` true))))

(fn `SetColor`
  (bind _digits (`self.Digits`))
  (bind _digits_2 (`self.Digits`))
  (bind _digits_3 (`self.Digits`))
  (bind _returnvalue (`PrimitiveComponent.CreateDynamicMaterialInstance` (`self.Color Indicator`) 0 null "None"))
  (if (`self.Tutorial`)
    (switch `/Game/Blueprints/Enums/ETutorialStage` "NewEnumerator0")
    (else
      (switch `/Game/Blueprints/Enums/EGameMutator` (`/Game/Blueprints/Blueprints/Gamemode_Manager/BP_GameManager.GameMutator` (`self.GameManagerRef`))
        (:`NewEnumerator0`
          ;[1 1 1] Make sure all values are different for better colors
          (bind _output_get (set `self.Red` (`|GetArrayItem` _digits_2 (`KismetMathLibrary.RandomInteger` (`KismetArrayLibrary.Array_Length` _digits_2)))))
          (`KismetArrayLibrary.Array_RemoveItem` (`self.Digits`) _output_get)
          (bind _output_get_2 (set `self.Green` (`|GetArrayItem` _digits_3 (`KismetMathLibrary.RandomInteger` (`KismetArrayLibrary.Array_Length` _digits_3)))))
          (`KismetArrayLibrary.Array_RemoveItem` (`self.Digits`) _output_get_2)
          (bind _output_get_3 (set `self.Blue` (`|GetArrayItem` _digits (`KismetMathLibrary.RandomInteger` (`KismetArrayLibrary.Array_Length` _digits)))))
          (`KismetArrayLibrary.Array_RemoveItem` (`self.Digits`) _output_get_3)
          ;[1 1 1] Readd all Digits
          (`KismetArrayLibrary.Array_Add` (`self.Digits`) (`self.Red`))
          (`KismetArrayLibrary.Array_Add` (`self.Digits`) (`self.Green`))
          (`KismetArrayLibrary.Array_Add` (`self.Digits`) (`self.Blue`))
          ;[1 1 1] Create RGB Value
          (bind _output_get_4 (set `self.Color` (make `LinearColor` (/ (`KismetMathLibrary.Conv_IntToDouble` (* (`self.Red`) 50)) 255.0) (/ (`KismetMathLibrary.Conv_IntToDouble` (* (`self.Green`) 50)) 255.0) (/ (`KismetMathLibrary.Conv_IntToDouble` (* (`self.Blue`) 50)) 255.0) 1.0)))
          (`MaterialInstanceDynamic.SetVectorParameterValue` _returnvalue "Color" _output_get_4))
        (:`NewEnumerator3`
          ;[1 1 1] Create Monochrome Values
          (set `self.Red` (`KismetMathLibrary.RandomInteger` 6))
          (bind _output_get_5 (set `self.Color` (make `LinearColor` (/ (`KismetMathLibrary.Conv_IntToDouble` (* (`self.Red`) 50)) 255.0) 0.0 0.0 1.0)))
          (`MaterialInstanceDynamic.SetVectorParameterValue` _returnvalue "Color" _output_get_5))
        (:`NewEnumerator4`
          (set `self.Green` (`KismetMathLibrary.RandomInteger` 6))
          (bind _output_get_6 (set `self.Color` (make `LinearColor` 0.0 (/ (`KismetMathLibrary.Conv_IntToDouble` (* (`self.Green`) 50)) 255.0) 0.0 1.0)))
          (`MaterialInstanceDynamic.SetVectorParameterValue` _returnvalue "Color" _output_get_6))
        (:`NewEnumerator5`
          (set `self.Blue` (`KismetMathLibrary.RandomInteger` 6))
          (bind _output_get_7 (set `self.Color` (make `LinearColor` 0.0 0.0 (/ (`KismetMathLibrary.Conv_IntToDouble` (* (`self.Blue`) 50)) 255.0) 1.0)))
          (`MaterialInstanceDynamic.SetVectorParameterValue` _returnvalue "Color" _output_get_7))))))

(fn `UserConstructionScript`)