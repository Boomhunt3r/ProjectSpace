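; BP_Storage is a four-board storage mechanism that shifts its boards downward when a Cube-tagged actor enters the move trigger.
; Each move records board positions, then a timeline lerps all four down one step.
; A separate Teleport_Board event sends the first board whose destination is near the bottom point to a reset location.
; BeginPlay caches all BP_TowerBase actors, but the cube-start logic that would target them is disconnected.
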(event `Move_Storage`
  ;[1 1 1] Move Storage
  (`self.Get Start and Destination`)
  (bind (_direction _0_1) (`Timeline|Lerp 0-1` :!via `PlayFromStart`)
    (:`Update`
      (`|ExecutionSequence`
        (:`then_0`
          (`self.NewFunction_0` _0_1 (`self.Board_01`) (`self.Board_01_StartLocation`) (`self.Board_01_Destination`)))
        (:`then_1`
          (`self.NewFunction_0` _0_1 (`self.Board_02`) (`self.Board_02_StartLocation`) (`self.Board_02_Destination`)))
        (:`then_2`
          (`self.NewFunction_0` _0_1 (`self.Board_03`) (`self.Board_03_StartLocation`) (`self.Board_03_Destination`)))
        (:`then_3`
          (`self.NewFunction_0` _0_1 (`self.Board_04`) (`self.Board_04_StartLocation`) (`self.Board_04_Destination`)))))))

(event `Teleport_Board`
  (bind _teleport_board_to (`self.Teleport Board to`))
  ;[1 1 1] Move Storage
  ;;[1 1 1] Check for Teleport
  (if (== (`self.Board_01_Destination`) (65.0 0.0 -130.0) :`ErrorTolerance` 20.0)
    (`SceneComponent.K2_SetRelativeLocation` (`self.Board_01`) _teleport_board_to false false)
    (elif (== (`self.Board_02_Destination`) (65.0 0.0 -130.0) :`ErrorTolerance` 20.0)
      (`SceneComponent.K2_SetRelativeLocation` (`self.Board_02`) _teleport_board_to false false)
      (elif (== (`self.Board_03_Destination`) (65.0 0.0 -130.0) :`ErrorTolerance` 20.0)
        (`SceneComponent.K2_SetRelativeLocation` (`self.Board_03`) _teleport_board_to false false)
        (elif (== (`self.Board_04_Destination`) (65.0 0.0 -130.0) :`ErrorTolerance` 20.0)
          (`SceneComponent.K2_SetRelativeLocation` (`self.Board_04`) _teleport_board_to false false))))))

(event `Launch Cube`)

(event `self.ReceiveBeginPlay`
  (bind _outactors (`GameplayStatics.GetAllActorsOfClass` "/Game/Blueprints/Blueprints/Tower/BP_TowerBase.BP_TowerBase_C"))
  (set `self.Tower Ref` _outactors))

(event `self.Trigger_Start Cube.OnComponentBeginOverlap`
  (params (OverlappedComponent :type "PrimitiveComponent Object Reference") (OtherActor :type "Actor Object Reference") (OtherComp :type "PrimitiveComponent Object Reference") (OtherBodyIndex :type Integer) (bFromSweep :type Boolean) (SweepResult :type "HitResult Structure (by ref)")))

(event `self.Trigger_MoveStorage.OnComponentBeginOverlap`
  (params (OverlappedComponent :type "PrimitiveComponent Object Reference") (OtherActor :type "Actor Object Reference") (OtherComp :type "PrimitiveComponent Object Reference") (OtherBodyIndex :type Integer) (bFromSweep :type Boolean) (SweepResult :type "HitResult Structure (by ref)"))
  (if (`self.ActorHasTag` OtherActor "Cube")
    (`self.Move_Storage`)))

(fn `Get Start and Destination`
  (bind _relativelocation (`SceneComponent.RelativeLocation` (`self.Board_04`)))
  (bind _relativelocation_2 (`SceneComponent.RelativeLocation` (`self.Board_01`)))
  (bind _relativelocation_3 (`SceneComponent.RelativeLocation` (`self.Board_02`)))
  (bind _relativelocation_4 (`SceneComponent.RelativeLocation` (`self.Board_03`)))
  (set `self.Board_01_StartLocation` _relativelocation_2)
  (set `self.Board_01_Destination` (- _relativelocation_2 (0.0 0.0 130.0)))
  (set `self.Board_02_StartLocation` _relativelocation_3)
  (set `self.Board_02_Destination` (- _relativelocation_3 (0.0 0.0 130.0)))
  (set `self.Board_03_StartLocation` _relativelocation_4)
  (set `self.Board_03_Destination` (- _relativelocation_4 (0.0 0.0 130.0)))
  (set `self.Board_04_StartLocation` _relativelocation)
  (set `self.Board_04_Destination` (- _relativelocation (0.0 0.0 130.0))))

(fn `NewFunction_0`
  (params (Lerp :type "Float (double-precision)") (Board :type "SceneComponent Object Reference") (Start :type "Vector Structure") (Destination :type "Vector Structure"))
  (`SceneComponent.K2_SetRelativeLocation` Board (`KismetMathLibrary.VLerp` Start Destination Lerp) false false))

(fn `UserConstructionScript`)