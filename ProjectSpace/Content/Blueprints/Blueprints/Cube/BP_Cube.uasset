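; Colored cube actor that moves along the Y axis once started, destroys overlapping bullets and can show a color stats widget.
; It starts with a random stepped RGB color on a dynamic material.
; ChangeColor lets Paint or Erase towers add or subtract clamped channel amounts.
; Pushing a channel out of range marks the cube cracked, and overflowing an already cracked cube calls EndGame on BP_GameManager.
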(event `self.ReceiveBeginPlay`
  ;[1 1 1] BeginPlay
  (`self.SetColor`)
  (bind _asui_cube (cast `/Game/UI/UI_Cube` (`WidgetComponent.GetUserWidgetObject` (`self.Widget`))))
  (`/Game/UI/UI_Cube.unique owner` _asui_cube self)
  (bind _returnvalue (`GameplayStatics.GetActorOfClass` "/Game/Blueprints/Blueprints/Manager/BP_GameManager.BP_GameManager_C"))
  (set `self.GameManagerRef` _returnvalue)
  (set `self.OrgMovementSpeed` (`self.MovementSpeed`)))

(event `self.ReceiveActorBeginOverlap`
  (params (OtherActor :type "Actor Object Reference"))
  ;[1 1 1] Destroy Bullet
  (if (`self.ActorHasTag` OtherActor "Bullet")
    (`self.K2_DestroyActor` OtherActor)))

(event `self.ReceiveTick`
  (params (DeltaSeconds :type "Float (single-precision)"))
  (bind _cube (`self.Cube`))
  (bind (_returnvalue_x _returnvalue_y _returnvalue_z) (`KismetMathLibrary.BreakVector` (`SceneComponent.K2_GetComponentLocation` _cube)))
  (bind (_returnvalue_x_2 _returnvalue_y_2) (`KismetMathLibrary.BreakVector` (+ (* (`KismetMathLibrary.Vector_Right`) (`self.MovementSpeed`)) (`SceneComponent.K2_GetComponentLocation` _cube))))
  ;[1 1 1] Move
  (if (`self.CanMove`)
    (`SceneComponent.K2_SetWorldLocation` (`self.Cube`) (`KismetMathLibrary.MakeVector` _returnvalue_x _returnvalue_y_2 _returnvalue_z) false false)))

(event `Start Cube`
  ;[1 1 1] Start Cube from Storage
  (if (== (`self.MovementSpeed`) 0.0)
    _
    (else
      _))
  (set `self.MovementSpeed` (* 1.0 (`self.Multiplier`)))
  (set `self.CanMove` true)
  (set `self.MovementSpeed` (`self.MovementSpeed`)))

(event `Show Color Stats`
  ;[1 1 1] Start Cube from Storage
  (`SceneComponent.SetVisibility` (`self.Widget`) true false))

(fn `ChangeColor`
  (params (Red :type Integer) (Green :type Integer) (Blue :type Integer) (TowerType :type "/Game/Blueprints/Enums/ETowerType Enum" :default "NewEnumerator0"))
  (locals (GivenRed :type Integer) (GivenGreen :type Integer) (GivenBlue :type Integer))
  (bind _cube (`self.Cube`))
  (bind _returnvalue (- (`self.Blue`) (`local.GivenBlue`)))
  (bind _returnvalue_2 (- (`self.Red`) (`local.GivenRed`)))
  (bind _returnvalue_3 (- (`self.Green`) (`local.GivenGreen`)))
  (bind _returnvalue_4 (+ (`self.Red`) (`local.GivenRed`)))
  (bind _returnvalue_5 (+ (`self.Green`) (`local.GivenGreen`)))
  (bind _returnvalue_6 (+ (`self.Blue`) (`local.GivenBlue`)))
  (set `local.GivenRed` Red)
  (set `local.GivenGreen` Green)
  (set `local.GivenBlue` Blue)
  (bind _returnvalue_7 (`PrimitiveComponent.CreateDynamicMaterialInstance` _cube 0 (`PrimitiveComponent.GetMaterial` _cube 0) "None"))
  (set `self.Mat` _returnvalue_7)
  (switch `/Game/Blueprints/Enums/ETowerType` TowerType
    (:`NewEnumerator1`
      (if (`self.hasCrack`)
        (set `self.2ndtime` true))
      (if (> _returnvalue_4 5)
        (set `self.hasCrack` true)
        (if (`self.2ndtime`)
          (`/Game/Blueprints/Blueprints/Manager/BP_GameManager.End Game` (`self.GameManagerRef`) true)
          (else
            (if (> _returnvalue_5 5) :!label _label
              (set `self.hasCrack` true)
              (if (`self.2ndtime`)
                (`/Game/Blueprints/Blueprints/Manager/BP_GameManager.End Game` (`self.GameManagerRef`) true)
                (else
                  (if (> _returnvalue_6 5) :!label _label_2
                    (set `self.hasCrack` true)
                    (if (`self.2ndtime`)
                      (`/Game/Blueprints/Blueprints/Manager/BP_GameManager.End Game` (`self.GameManagerRef`) true)
                      (else
                        (bind _output_get (set `self.Red` (`KismetMathLibrary.Clamp` _returnvalue_4 0 5) :!label _label_3))
                        (bind _output_get_2 (set `self.Green` (`KismetMathLibrary.Clamp` _returnvalue_5 0 5)))
                        (bind _output_get_3 (set `self.Blue` (`KismetMathLibrary.Clamp` _returnvalue_6 0 5)))
                        (bind _output_get_4 (set `self.Color` (make `LinearColor` (/ (`KismetMathLibrary.Conv_IntToDouble` (* _output_get 50)) 255.0) (/ (`KismetMathLibrary.Conv_IntToDouble` (* _output_get_2 50)) 255.0) (/ (`KismetMathLibrary.Conv_IntToDouble` (* _output_get_3 50)) 255.0) 1.0)))
                        (`MaterialInstanceDynamic.SetVectorParameterValue` (`self.Mat`) "Color" _output_get_4)))
                    (else
                      (set `self.2ndtime` false)
                      (goto _label_3)))))
              (else
                (goto _label_2)))))
        (else
          (goto _label))))
    (:`NewEnumerator2`
      (if (`self.hasCrack`)
        (set `self.2ndtime` true))
      (if (< _returnvalue_2 0)
        (set `self.hasCrack` true)
        (if (`self.2ndtime`)
          (`/Game/Blueprints/Blueprints/Manager/BP_GameManager.End Game` (`self.GameManagerRef`) true)
          (else
            (if (< _returnvalue_3 0) :!label _label_4
              (set `self.hasCrack` true)
              (if (`self.2ndtime`)
                (`/Game/Blueprints/Blueprints/Manager/BP_GameManager.End Game` (`self.GameManagerRef`) true)
                (else
                  (if (< _returnvalue 0) :!label _label_5
                    (set `self.hasCrack` true)
                    (if (`self.2ndtime`)
                      (`/Game/Blueprints/Blueprints/Manager/BP_GameManager.End Game` (`self.GameManagerRef`) true)
                      (else
                        (bind _output_get_5 (set `self.Red` (`KismetMathLibrary.Clamp` _returnvalue_2 0 5) :!label _label_6))
                        (bind _output_get_6 (set `self.Green` (`KismetMathLibrary.Clamp` _returnvalue_3 0 5)))
                        (bind _output_get_7 (set `self.Blue` (`KismetMathLibrary.Clamp` _returnvalue 0 5)))
                        (bind _output_get_8 (set `self.Color` (make `LinearColor` (/ (`KismetMathLibrary.Conv_IntToDouble` (* _output_get_5 50)) 255.0) (/ (`KismetMathLibrary.Conv_IntToDouble` (* _output_get_6 50)) 255.0) (/ (`KismetMathLibrary.Conv_IntToDouble` (* _output_get_7 50)) 255.0) 1.0)))
                        (`MaterialInstanceDynamic.SetVectorParameterValue` (`self.Mat`) "Color" _output_get_8)))
                    (else
                      (goto _label_6)))))
              (else
                (goto _label_5)))))
        (else
          (goto _label_4))))))

(fn `SetColor`
  (bind _returnvalue (`PrimitiveComponent.CreateDynamicMaterialInstance` (`self.Cube`) 0 null "None"))
  (`|ExecutionSequence`
    (:`then_0`
      (bind _output_get (set `self.Red` (`KismetMathLibrary.RandomInteger` 6))))
    (:`then_1`
      (bind _output_get_2 (set `self.Green` (`KismetMathLibrary.RandomInteger` 6))))
    (:`then_2`
      (bind _output_get_3 (set `self.Blue` (`KismetMathLibrary.RandomInteger` 6))))
    (:`then_3`
      (`MaterialInstanceDynamic.SetVectorParameterValue` _returnvalue "Color" (make `LinearColor` (/ (`KismetMathLibrary.Conv_IntToDouble` (* _output_get 50)) 255.0) (/ (`KismetMathLibrary.Conv_IntToDouble` (* _output_get_2 50)) 255.0) (/ (`KismetMathLibrary.Conv_IntToDouble` (* _output_get_3 50)) 255.0) 1.0)))))

(fn `UserConstructionScript`)