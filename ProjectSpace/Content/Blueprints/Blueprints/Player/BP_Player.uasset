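; BP_Player is the player Blueprint that owns the game's screen UI and the entry point for starting play.
; BeginPlay creates all menu and HUD widgets, adds them to the viewport up front and hides all but the main menu.
; StartGame tells the level's BP_CubeManager to start and reveals the HUD.
; Right mouse is forwarded as a left-click through a WidgetInteraction component.
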(event `Start Game`
  (bind _returnvalue (`GameplayStatics.GetActorOfClass` "/Game/Blueprints/Blueprints/Cube/BP_CubeManager.BP_CubeManager_C"))
  (`/Game/Blueprints/Blueprints/Cube/BP_CubeManager.Start Game` _returnvalue)
  (`Widget.SetVisibility` (`self.UI_HUD`) "Visible"))

(event `self.ReceiveBeginPlay`
  (`|ExecutionSequence`
    (:`then_0`
      (bind _returnvalue (`|CreateWidget` "/Game/UI/UI_HUD.UI_HUD_C"))
      (bind _output_get (set `self.UI_HUD` _returnvalue))
      (`UserWidget.AddToViewport` _output_get 0)
      (`Widget.SetVisibility` _output_get "Hidden"))
    (:`then_1`
      (bind _returnvalue_2 (`|CreateWidget` "/Game/UI/UI_MainMenu.UI_MainMenu_C"))
      (bind _output_get_2 (set `self.UI_MainMenu` _returnvalue_2))
      (`UserWidget.AddToViewport` _output_get_2 0))
    (:`then_2`
      (bind _returnvalue_3 (`|CreateWidget` "/Game/UI/UI_GameOver.UI_GameOver_C"))
      (bind _output_get_3 (set `self.UI_GameOver` _returnvalue_3))
      (`UserWidget.AddToViewport` _output_get_3 0)
      (`Widget.SetVisibility` _output_get_3 "Hidden"))
    (:`then_3`
      (bind _returnvalue_4 (`|CreateWidget` "/Game/UI/UI_Gamemodes.UI_Gamemodes_C"))
      (bind _output_get_4 (set `self.UI_Gamemodes` _returnvalue_4))
      (`UserWidget.AddToViewport` _output_get_4 0)
      (`Widget.SetVisibility` _output_get_4 "Hidden"))
    (:`then_4`
      (bind _returnvalue_5 (`|CreateWidget` "/Game/UI/UI_Options.UI_Options_C"))
      (bind _output_get_5 (set `self.UI_Options` _returnvalue_5))
      (`UserWidget.AddToViewport` _output_get_5 0)
      (`Widget.SetVisibility` _output_get_5 "Hidden"))
    (:`then_5`
      (bind _returnvalue_6 (`|CreateWidget` "/Game/UI/UI_Scores.UI_Scores_C"))
      (bind _output_get_6 (set `self.UI_Scores` _returnvalue_6))
      (`UserWidget.AddToViewport` _output_get_6 0)
      (`Widget.SetVisibility` _output_get_6 "Hidden"))
    (:`then_6`
      (bind _returnvalue_7 (`|CreateWidget` "/Game/UI/UI_Share.UI_Share_C"))
      (bind _output_get_7 (set `self.UI_Share` _returnvalue_7))
      (`UserWidget.AddToViewport` _output_get_7 0)
      (`Widget.SetVisibility` _output_get_7 "Hidden"))))

(event `Key|RightMouseButton`
  (params (Key :type "Key Structure"))
  (bind _widgetinteraction (`self.WidgetInteraction`))
  (:`Pressed`
    (`WidgetInteractionComponent.PressPointerKey` _widgetinteraction "LeftMouseButton"))
  (:`Released`
    (`WidgetInteractionComponent.ReleasePointerKey` _widgetinteraction "LeftMouseButton")))

(fn `UserConstructionScript`)