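; Spline tool actor that scatters static meshes along a path at a set spacing, built in the Construction Script.
; It first snaps each spline point to the surface with visibility line traces, then adds a mesh component per step if SpawnObjects is on.
; Each component gets a random mesh, materials and scale jitter, with rotation either following the spline or randomized.
; Flags can hide meshes at construction or the whole root at BeginPlay.
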(event `self.ReceiveBeginPlay`
  (if (`self.Hide in Game`)
    (`SceneComponent.SetVisibility` (`self.DefaultSceneRoot`) false true)))

(fn `UserConstructionScript`
  (bind (_meshoffset_x _meshoffset_y _meshoffset_z) (`KismetMathLibrary.BreakVector` (`self.MeshOffset`)))
  (bind (_meshscale_x _meshscale_y _meshscale_z) (`KismetMathLibrary.BreakVector` (`self.MeshScale`)))
  (bind (_max_randomrotation_x _max_randomrotation_y _max_randomrotation_z) (`KismetMathLibrary.BreakVector` (`self.Max_RandomRotation`)))
  (bind _material (`self.Material`))
  (bind _meshes_to_spawn (`self.Meshes to spawn`))
  (bind (_snapthreshold_x_x _snapthreshold_x_y _snapthreshold_x_z) (`KismetMathLibrary.BreakVector` (`self.SnapThreshold_X`)))
  (bind (_meshrotation_roll _meshrotation_pitch _meshrotation_yaw) (`KismetMathLibrary.BreakRotator` (`self.MeshRotation`)))
  (bind (_maxrandomscale_x _maxrandomscale_y _maxrandomscale_z) (`KismetMathLibrary.BreakVector` (`self.MaxRandomScale`)))
  (bind (_rotation_allignment_x _rotation_allignment_y _rotation_allignment_z) (`KismetMathLibrary.BreakVector` (`self.Rotation_Allignment`)))
  (bind _output (`|GetArrayItem` _material (`KismetMathLibrary.RandomInteger` (`KismetArrayLibrary.Array_Length` _material))))
  (bind _returnvalue (`KismetMathLibrary.MakeVector` (+ _meshscale_x (`KismetMathLibrary.RandomFloatInRange` (* _maxrandomscale_x -1.0) _maxrandomscale_x)) (+ _meshscale_y (`KismetMathLibrary.RandomFloatInRange` (* _maxrandomscale_y -1.0) _maxrandomscale_y)) (+ _meshscale_z (`KismetMathLibrary.RandomFloatInRange` (* _maxrandomscale_z -1.0) _maxrandomscale_z))))
  (`|ExecutionSequence`
    (:`then_0`
      ;[1 1 1] Snap Spline to Surface
      (for _index (range (`SplineComponent.GetNumberOfSplinePoints` (`self.Spline`)))
        (bind (_returnvalue_x _returnvalue_y _returnvalue_z) (`KismetMathLibrary.BreakVector` (`SplineComponent.GetLocationAtSplinePoint` (`self.Spline`) _index "World")))
        (bind (_returnvalue_x_2 _returnvalue_y_2 _returnvalue_z_2) (`KismetMathLibrary.BreakVector` (`SplineComponent.GetLocationAtSplinePoint` (`self.Spline`) _index "World")))
        (bind (_outhit _returnvalue_2) (`KismetSystemLibrary.LineTraceSingle` :`Start` (`KismetMathLibrary.MakeVector` (+ _snapthreshold_x_x _returnvalue_x) (+ _returnvalue_y _snapthreshold_x_y) (+ _returnvalue_z _snapthreshold_x_z)) :`End` (`KismetMathLibrary.MakeVector` (- _returnvalue_x_2 _snapthreshold_x_x) (- _returnvalue_y_2 _snapthreshold_x_y) (- _returnvalue_z_2 _snapthreshold_x_z)) :`TraceChannel` "TraceTypeQuery1" :`DrawDebugType` "ForDuration"))
        (if _returnvalue_2
          (`SplineComponent.SetLocationAtSplinePoint` (`self.Spline`) _index (`.Location` (`GameplayStatics.BreakHitResult` _outhit)) "World" true))))
    (:`then_1`
      (if (`self.Spawn Objects`)
        (for _index_2 (range (+ (`KismetMathLibrary.FTrunc` (/ (`SplineComponent.GetSplineLength` (`self.Spline`)) (* (`self.Distance Between Meshes`) 100.0))) 1))
          (bind _returnvalue_3 (`AddComponent|NODE_AddStaticMeshComponent-1`))
          (`SceneComponent.SetMobility` _returnvalue_3 (`self.Mobility`))
          (if (`self.Follow Spline Rotation?`)
            (bind _returnvalue_4 (* _index_2 (* (`self.Distance Between Meshes`) 100.0)))
            (bind (_returnvalue_x_3 _returnvalue_y_3 _returnvalue_z_3) (`KismetMathLibrary.BreakVector` (`SplineComponent.GetLocationAtDistanceAlongSpline` (`self.Spline`) _returnvalue_4 "World")))
            (bind _returnvalue_5 (`KismetMathLibrary.MakeVector` (+ _meshoffset_x _returnvalue_x_3) (+ _meshoffset_y _returnvalue_y_3) (+ _returnvalue_z_3 _meshoffset_z)))
            (bind (_returnvalue_roll _returnvalue_pitch _returnvalue_yaw) (`KismetMathLibrary.BreakRotator` (`SplineComponent.GetRotationAtDistanceAlongSpline` (`self.Spline`) _returnvalue_4 "World")))
            ;[1 1 1] fix projection
            (`SceneComponent.K2_SetWorldTransform` _returnvalue_3 (`KismetMathLibrary.MakeTransform` _returnvalue_5 (`KismetMathLibrary.MakeRotator` (+ _returnvalue_roll _rotation_allignment_x) (+ _returnvalue_pitch _rotation_allignment_y) (+ _returnvalue_yaw _rotation_allignment_z)) _returnvalue) false false)
            (else
              (`SceneComponent.K2_SetWorldTransform` _returnvalue_3 (`KismetMathLibrary.MakeTransform` _returnvalue_5 (`KismetMathLibrary.MakeRotator` (+ _meshrotation_roll (`KismetMathLibrary.RandomFloatInRange` (* _max_randomrotation_x -1.0) _max_randomrotation_x)) (+ _meshrotation_pitch (`KismetMathLibrary.RandomFloatInRange` (* _max_randomrotation_y -1.0) _max_randomrotation_y)) (+ _meshrotation_yaw (`KismetMathLibrary.RandomFloatInRange` (* _max_randomrotation_z -1.0) _max_randomrotation_z))) _returnvalue) false false)))
          ;[1 1 1] Setting Meshes
          (`StaticMeshComponent.SetStaticMesh` _returnvalue_3 (`|GetArrayItem` _meshes_to_spawn (`KismetMathLibrary.RandomInteger` (`KismetArrayLibrary.Array_Length` _meshes_to_spawn))))
          ;[1 1 1] Setting collision
          (`PrimitiveComponent.SetCollisionEnabled` _returnvalue_3 (`self.Collision`))
          ;[1 1 1] Setting Materials
          (`PrimitiveComponent.SetMaterial` _returnvalue_3 0 _output)
          (`PrimitiveComponent.SetMaterial` _returnvalue_3 1 _output)
          (`PrimitiveComponent.SetMaterial` _returnvalue_3 2 _output)
          (`PrimitiveComponent.SetMaterial` _returnvalue_3 3 _output)
          (`PrimitiveComponent.SetMaterial` _returnvalue_3 4 _output)
          (`PrimitiveComponent.SetMaterial` _returnvalue_3 5 _output)
          ;[1 1 1] Setting Decal Activation
          (`PrimitiveComponent.SetReceivesDecals` _returnvalue_3 false)
          (if (`self.Hide in Editor`)
            (`SceneComponent.SetVisibility` _returnvalue_3 false false)))))))