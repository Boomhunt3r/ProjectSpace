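; BP_GameManager runs the round flow for a color cube game: start, game over, reset and highscore saving.
; On BeginPlay it caches the player, cube manager, goal, storage, target RGB and teleport actors, and loads the highscore via the game instance.
; Starting sets the goal color, hides the RGB target for certain mutators and starts a looping countdown in Rush mode.
; Timeout or wrong color shows game over and freezes all cubes.
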(event `self.ReceiveBeginPlay`
  ;[1 1 1] Start Up
  (`|ExecutionSequence`
    (:`then_0`
      (bind _returnvalue (`GameplayStatics.GetActorOfClass` "/Game/Blueprints/Blueprints/Player/BP_Player.BP_Player_C"))
      (set `self.PlayerRef` _returnvalue))
    (:`then_1`
      (bind _returnvalue_2 (`GameplayStatics.GetActorOfClass` "/Game/Blueprints/Blueprints/Cube/BP_CubeManager.BP_CubeManager_C"))
      (set `self.CubeManagerRef` _returnvalue_2))
    (:`then_2`
      (bind _returnvalue_3 (`GameplayStatics.GetActorOfClass` "/Game/Blueprints/Blueprints/Goal/BP_Goal.BP_Goal_C"))
      (set `self.GoalRef` _returnvalue_3))
    (:`then_3`
      (bind _returnvalue_4 (`GameplayStatics.GetActorOfClass` "/Game/Blueprints/Blueprints/BP_Storage.BP_Storage_C"))
      (set `self.Storage Ref` _returnvalue_4))
    (:`then_4`
      (bind _returnvalue_5 (`GameplayStatics.GetActorOfClass` "/Game/UI/BP_UI_TargetRGB.BP_UI_TargetRGB_C"))
      (set `self.TargetRGBRef` _returnvalue_5))
    (:`then_5`
      (bind _returnvalue_6 (`GameplayStatics.GetActorOfClass` "/Game/Blueprints/Blueprints/Goal/BP_TpBack.BP_TpBack_C"))
      (set `self.TP_Back Ref` _returnvalue_6))
    (:`then_6`
      (bind _asbp_game_instane (cast `/Game/Blueprints/Blueprints/BP_GameInstane` (`GameplayStatics.GetGameInstance`)))
      (bind _output_get (set `self.GameInstanceRef` _asbp_game_instane))
      (set `self.Highscore` (`/Game/Blueprints/Blueprints/BP_SaveGame.Highscore` (`/Game/Blueprints/Blueprints/BP_GameInstane.SaveGameRef` _output_get))))))

(event `Start Game`
  ;[1 1 1] Start Game
  (`/Game/Blueprints/Blueprints/Cube/BP_CubeManager.Start Game` (`self.CubeManagerRef`))
  (`|ExecutionSequence`
    (:`then_0`
      (`/Game/Blueprints/Blueprints/Goal/BP_Goal.SetColor` (`self.GoalRef`))
      ;;[1 1 1] Hide Target RGB Value for some Mutators
      (switch `/Game/Blueprints/Enums/EGameMutator` (`self.GameMutator`)
        (:`NewEnumerator2`
          _)
        (:`NewEnumerator3`
          _)
        (:`NewEnumerator4`
          _)
        (:`NewEnumerator5`
          _))
      (`Widget.SetVisibility` (`WidgetComponent.GetUserWidgetObject` (`/Game/UI/BP_UI_TargetRGB.Widget` (`self.TargetRGBRef`))) "Hidden"))
    (:`then_1`
      (switch `/Game/Blueprints/Enums/EGameMode` (`self.GameMode`)
        (:`NewEnumerator2`
          (set `self.Timer (Rush)` 20)
          (`self.Start Timer (Rush only)`))))))

(event `Start Timer (Rush only)`
  (bind _returnvalue (`KismetSystemLibrary.K2_SetTimer` null "Rush Timer" 1.0 true)))

(event `self.ReceiveTick`
  (params (DeltaSeconds :type "Float (single-precision)"))
  (`KismetSystemLibrary.PrintString` (`KismetStringLibrary.Conv_IntToString` (`self.Timer (Rush)`))))

(event `Timer Ended (Rush)`
  (bind _playerref (`self.PlayerRef`))
  (bind _ui_gameover (`/Game/Blueprints/Blueprints/Player/BP_Player.UI_GameOver` _playerref))
  ;[1 1 1] End Game
  (`|ExecutionSequence`
    (:`then_0`
      (`KismetSystemLibrary.K2_ClearAndInvalidateTimerHandle` (stale `Start Timer (Rush only)` _returnvalue)))
    (:`then_1`
      (set `/Game/Blueprints/Blueprints/Player/BP_Player.isAlive` false _playerref :!label _label)
      (`Widget.SetVisibility` (`/Game/Blueprints/Blueprints/Player/BP_Player.UI_HUD` _playerref) "Hidden")
      (`Widget.SetVisibility` _ui_gameover "Visible")
      (`/Game/UI/Menus/UI_GameOver.Start GameOverAnimation` _ui_gameover)
      (for _array_element (`/Game/Blueprints/Blueprints/Cube/BP_CubeManager.Cubes` (`self.CubeManagerRef`))
        (set `/Game/Blueprints/Blueprints/Cube/BP_Cube.CanMove` false _array_element)))))

(event `End Game`
  (params (WrogColor :type Boolean))
  ;[1 1 1] End Game
  (if WrogColor
    (goto _label)))

(event `SaveHighscore`
  (bind _gameinstanceref (`self.GameInstanceRef`))
  (bind _savegameref (`/Game/Blueprints/Blueprints/BP_GameInstane.SaveGameRef` _gameinstanceref))
  ;[1 1 1] Save Score
  (set `/Game/Blueprints/Blueprints/BP_SaveGame.Highscore` (`self.Highscore`) _savegameref)
  (`GameplayStatics.SaveGameToSlot` _savegameref (`/Game/Blueprints/Blueprints/BP_GameInstane.SaveGameName` _gameinstanceref)))

(event `Reset Game`
  (`/Game/Blueprints/Blueprints/BP_Storage.Teleport_Board` (`self.Storage Ref`))
  (`/Game/Blueprints/Blueprints/Goal/BP_TpBack.Rest Current Cube` (`self.TP_Back Ref`) (`/Game/Blueprints/Blueprints/Cube/BP_CubeManager.Current Cube` (`self.CubeManagerRef`)))
  (`self.Start Game`))

(fn `Rush Timer`
  (locals (done :type Boolean))
  (bind _result (`/Engine/EditorBlueprintResources/StandardMacros.DecrementInt` (`self.Timer (Rush)`))
    (:`  `
      (if (== _result 0)
        (`self.Timer Ended (Rush)`)))))

(fn `UserConstructionScript`)