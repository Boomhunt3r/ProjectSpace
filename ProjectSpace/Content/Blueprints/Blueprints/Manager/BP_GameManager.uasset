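; Game manager Blueprint for a color-matching game with modes and mutators, coordinating the player, cube manager, goal and target RGB widget.
; BeginPlay caches those actors and loads the highscore from the game instance's save object, which SaveHighscore writes back to its slot.
; StartGame sets the goal color, hiding the RGB target for Hardcore and Monochrome mutators; ResetGame restores Arcade counter and cube speeds.
; EndGame handles wrong-color game over.
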(event `self.ReceiveBeginPlay`
  (bind _returnvalue (`GameplayStatics.GetActorOfClass` "/Game/Blueprints/Blueprints/Player/BP_Player.BP_Player_C"))
  (set `self.PlayerRef` _returnvalue)
  (bind _returnvalue_2 (`GameplayStatics.GetActorOfClass` "/Game/Blueprints/Blueprints/Cube/BP_CubeManager.BP_CubeManager_C"))
  (set `self.CubeManagerRef` _returnvalue_2)
  (bind _returnvalue_3 (`GameplayStatics.GetActorOfClass` "/Game/Blueprints/Blueprints/Trigger/BP_Goal.BP_Goal_C"))
  (set `self.GoalRef` _returnvalue_3)
  (bind _asbp_game_instane (cast `/Game/Blueprints/Blueprints/BP_GameInstane` (`GameplayStatics.GetGameInstance`)))
  (bind _output_get (set `self.GameInstanceRef` _asbp_game_instane))
  (set `self.Highscore` (`/Game/Blueprints/Blueprints/BP_SaveGame.Highscore` (`/Game/Blueprints/Blueprints/BP_GameInstane.SaveGameRef` _output_get)))
  (bind _returnvalue_4 (`GameplayStatics.GetActorOfClass` "/Game/UI/BP_UI_TargetRGB.BP_UI_TargetRGB_C"))
  (set `self.TargetRGBRef` _returnvalue_4))

(event `Selected Gamemode`
  (params (NewParam :type Boolean) (NewParam2 :type Boolean) (NewParam3 :type Boolean)))

(event `End Game`
  (params (WrogColor :type Boolean))
  (bind _playerref (`self.PlayerRef`))
  (bind _ui_gameover (`/Game/Blueprints/Blueprints/Player/BP_Player.UI_GameOver` _playerref))
  (if WrogColor
    (set `/Game/Blueprints/Blueprints/Player/BP_Player.isAlive` false _playerref)
    (`/Game/Blueprints/Blueprints/Cube/BP_CubeManager.EndGame` (`self.CubeManagerRef`))
    (`Widget.SetVisibility` (`/Game/Blueprints/Blueprints/Player/BP_Player.UI_HUD` _playerref) "Hidden")
    (`Widget.SetVisibility` _ui_gameover "Visible")
    (`/Game/UI/Menus/UI_GameOver.Start GameOverAnimation` _ui_gameover)))

(event `SaveHighscore`
  (bind _gameinstanceref (`self.GameInstanceRef`))
  (bind _savegameref (`/Game/Blueprints/Blueprints/BP_GameInstane.SaveGameRef` _gameinstanceref))
  (set `/Game/Blueprints/Blueprints/BP_SaveGame.Highscore` (`self.Highscore`) _savegameref)
  (`GameplayStatics.SaveGameToSlot` _savegameref (`/Game/Blueprints/Blueprints/BP_GameInstane.SaveGameName` _gameinstanceref)))

(fn `ResetGame`
  (switch `/Game/Blueprints/Enums/EGameMode` (`self.GameMode`)
    (:`NewEnumerator1`
      (set `/Game/Blueprints/Blueprints/Trigger/BP_Goal.Success Counter` 0 (`self.GoalRef`))
      (for _array_element (`/Game/Blueprints/Blueprints/Cube/BP_CubeManager.Cubes` (`self.CubeManagerRef`))
        (set `/Game/Blueprints/Blueprints/Cube/BP_Cube.MovementSpeed` (`/Game/Blueprints/Blueprints/Cube/BP_Cube.OrgMovementSpeed` _array_element) _array_element)))
    (:`NewEnumerator2`)))

(fn `StartGame`
  (`/Game/Blueprints/Blueprints/Trigger/BP_Goal.SetColor` (`self.GoalRef`))
  (switch `/Game/Blueprints/Enums/EGameMutator` (`self.GameMutator`)
    (:`NewEnumerator2`
      _)
    (:`NewEnumerator3`
      _)
    (:`NewEnumerator4`
      _)
    (:`NewEnumerator5`
      _))
  (`Widget.SetVisibility` (`WidgetComponent.GetUserWidgetObject` (`/Game/UI/BP_UI_TargetRGB.Widget` (`self.TargetRGBRef`))) "Hidden"))

(fn `UserConstructionScript`)