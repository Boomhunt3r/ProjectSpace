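; BP_TowerBase is a tower turret that tracks a target and fires BP_Bullet projectiles.
; While following, Tick restarts timelines that lerp the base's yaw toward the target and aim the gun with clamped pitch.
; Firesingleshot calls Shoot, then clears the cooldown flag when a timeline finishes.
; Shoot spawns the bullet and, while following, directly passes the tower's color and type to the target BP_Cube's ChangeColor.
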(event `self.ReceiveTick`
  (params (DeltaSeconds :type "Float (single-precision)"))
  (bind _base (`self.Base`))
  (bind _gun (`self.Gun`))
  (bind (_returnvalue_roll _returnvalue_pitch _returnvalue_yaw) (`KismetMathLibrary.BreakRotator` (`KismetMathLibrary.FindLookAtRotation` (`SceneComponent.K2_GetComponentLocation` _base) (`self.K2_GetActorLocation` (`self.Target Ref`)))))
  (if (`self.should follow Target`)
    ;[1 1 1] Base Rotation
    (bind (_direction _newtrack_0) (`Timeline|Timeline_0` :!via `PlayFromStart`)
      (:`Update`
        (bind (_returnvalue_roll_2 _returnvalue_pitch_2 _returnvalue_yaw_2) (`KismetMathLibrary.BreakRotator` (`KismetMathLibrary.RLerp` (`SceneComponent.K2_GetComponentRotation` _base) (`KismetMathLibrary.MakeRotator` _returnvalue_roll _returnvalue_pitch _returnvalue_yaw) _newtrack_0 true)))
        (`SceneComponent.K2_SetWorldRotation` (`self.Base`) (`KismetMathLibrary.MakeRotator` 0.0 0.0 _returnvalue_yaw_2) false false)
        ;[1 1 1] Gun Rotation
        (bind (_direction_2 _newtrack_0_2) (`Timeline|Timeline_1` :!via `PlayFromStart`)
          (:`Update`
            (bind (_returnvalue_roll_3 _returnvalue_pitch_3) (`KismetMathLibrary.BreakRotator` (`KismetMathLibrary.RLerp` (`SceneComponent.K2_GetComponentRotation` _gun) (`KismetMathLibrary.FindLookAtRotation` (`SceneComponent.K2_GetComponentLocation` _gun) (+ (`self.K2_GetActorLocation` (`self.Target Ref`)) (0.0 0.0 50.0))) _newtrack_0_2 true)))
            (`SceneComponent.K2_SetWorldRotation` (`self.Gun`) (`KismetMathLibrary.MakeRotator` 0.0 (`KismetMathLibrary.FClamp` _returnvalue_pitch_3 -20.0) _returnvalue_yaw_2) false false)))))))

(event `Fire single shot`
  (`self.Shoot`)
  (`Timeline|Timeline_2` :!via `PlayFromStart`
    (:`Finished`
      (set `self.Shoot on Cooldown` false))))

(fn `Set Color`
  (params (Red :type Integer) (Green :type Integer) (Blue :type Integer))
  (set `self.Red` Red)
  (set `self.Green` Green)
  (set `self.Blue` Blue))

(fn `Shoot`
  (bind (_returnvalue_location _returnvalue_rotation) (`KismetMathLibrary.BreakTransform` (`SceneComponent.K2_GetComponentToWorld` (`self.Gun`))))
  (`|SpawnActorFromClass` "/Game/Blueprints/Blueprints/Bullet/BP_Bullet.BP_Bullet_C" (`KismetMathLibrary.MakeTransform` (+ _returnvalue_location (`KismetMathLibrary.GetForwardVector` _returnvalue_rotation)) _returnvalue_rotation) "Undefined" "OverrideRootScale" null null)
  (if (`self.should follow Target`)
    (bind _asbp_cube (cast `/Game/Blueprints/Blueprints/Cube/BP_Cube` (`self.Target Ref`)))
    (`/Game/Blueprints/Blueprints/Cube/BP_Cube.ChangeColor` _asbp_cube (`self.Red`) (`self.Green`) (`self.Blue`) (`self.Type`))))

(fn `UserConstructionScript`)