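; BP_SpawnerManager runs round state across the BP_EnemySpawner actors in the level.
; On BeginPlay it gathers every spawner into an array and records the count.
; StartRound re-enables each spawner, resets its counters and flags, and clears the empty-spawner list.
; AddEmptySpawner records each exhausted spawner once and ends the round when that list's length matches the spawner count.
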(event `self.ReceiveBeginPlay`
  (bind _outactors (`GameplayStatics.GetAllActorsOfClass` "/Game/Blueprints/Old/EnemySpawner/BP_EnemySpawner.BP_EnemySpawner_C"))
  (bind _output_get (set `self.Spawner` _outactors))
  (set `self.SpawnerLength` (`KismetArrayLibrary.Array_Length` _output_get)))

(fn `AddEmptySpawner`
  (params (Spawner :type "/Game/Blueprints/Old/EnemySpawner/BP_EnemySpawner Object Reference"))
  (if (not (`KismetArrayLibrary.Array_Contains` (`self.EmptySpawner`) Spawner))
    (`KismetArrayLibrary.Array_Add` (`self.EmptySpawner`) Spawner)
    (if (== (`KismetArrayLibrary.Array_Length` (`self.Spawner`)) (`KismetArrayLibrary.Array_Length` (`self.EmptySpawner`)))
      (set `self.RoundStarted` false)
      (set `self.RoundOver` true))))

(fn `Start Round`
  (for _array_element (`self.Spawner`)
    (set `/Game/Blueprints/Old/EnemySpawner/BP_EnemySpawner.CanSpawn` true _array_element)
    (set `/Game/Blueprints/Old/EnemySpawner/BP_EnemySpawner.NoEnemy` false _array_element)
    (set `/Game/Blueprints/Old/EnemySpawner/BP_EnemySpawner.TotalSpawned` 0 _array_element))
  (set `self.RoundStarted` true)
  (set `self.RoundOver` false)
  (`KismetArrayLibrary.Array_Clear` (`self.EmptySpawner`)))

(fn `UserConstructionScript`)