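; BP_EnemySpawner is an enemy spawner actor that, while CanSpawn is set, spawns AI of EnemyClass at its root location.
; BeginPlay caches the BP_SpawnerManager, and Tick accumulates a timer against SpawnTime.
; Timer reset, enemy tracking and the spawn limit are disconnected, so spawning repeats every tick after the threshold.
; RemoveEnemyFromArray is an empty stub, with its manager notification also disconnected.
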(event `self.ReceiveBeginPlay`
  (bind _returnvalue (`GameplayStatics.GetActorOfClass` "/Game/Blueprints/Old/EnemySpawner/BP_SpawnerManager.BP_SpawnerManager_C"))
  (set `self.SpawnerManager` _returnvalue))

(event `self.ReceiveTick`
  (params (DeltaSeconds :type "Float (single-precision)"))
  (if (`self.CanSpawn`)
    (set `self.SpawnTimer` (+ DeltaSeconds (`self.SpawnTimer`)))
    (if (>= (`self.SpawnTimer`) (`self.SpawnTime`))
      (`AIBlueprintHelperLibrary.SpawnAIFromClass` (`self.Enemy Class`) null (`SceneComponent.K2_GetComponentLocation` (`self.DefaultSceneRoot`)) (struct) false null))))

(fn `RemoveEnemyFromArray`
  (params (EnemyToRemove :type "Object Object Reference"))
  (if true
    _))

(fn `UserConstructionScript`)