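; Tower-defense turret that tracks tagged enemies entering its Range-scaled collision and fires projectiles at the first target.
; Overlaps maintain the target list, which SortArray reorders to favor heavy or regular ground enemies by Heavy or MG weapon type.
; Tick line-traces for sight, then nested timelines turn base and pitch-clamped gun, accumulating time to spawn BP_TestProjectile with the tower's damage stats.
; UpdateTower shortens the fire interval for upgrade states.
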(event `self.ReceiveBeginPlay`
  (`SceneComponent.SetVisibility` (`self.Collision`) false false))

(event `self.ReceiveActorBeginOverlap`
  (params (OtherActor :type "Actor Object Reference"))
  ;[1 1 1] Is Enemy in Range?
  (if (`self.ActorHasTag` OtherActor (`self.EnemyTag`))
    (set `self.Enemy Is Near` true)
    (bind _output_get (set `self.Target` OtherActor))
    (`KismetArrayLibrary.Array_Add` (`self.Targets`) _output_get)
    (`self.SortArray`)))

(event `self.ReceiveActorEndOverlap`
  (params (OtherActor :type "Actor Object Reference"))
  ;[1 1 1] Is Enemy in Range?
  (if (`self.ActorHasTag` OtherActor (`self.EnemyTag`))
    (`self.RemoveFromArray` OtherActor)))

(event `self.ReceiveTick`
  (params (DeltaSeconds :type "Float (single-precision)"))
  (bind _targets (`self.Targets`))
  (bind _targets_2 (`self.Targets`))
  (bind _base (`self.Base`))
  (bind _gun (`self.Gun`))
  (bind (_returnvalue_location _returnvalue_rotation) (`KismetMathLibrary.BreakTransform` (`SceneComponent.K2_GetComponentToWorld` (`self.Gun`))))
  (`KismetSystemLibrary.Delay` 0.5)
  (if (`self.Enemy Is Near`)
    (bind _outhit (`KismetSystemLibrary.LineTraceSingle` :`Start` (`SceneComponent.K2_GetComponentLocation` (`self.Gun`)) :`End` (`self.K2_GetActorLocation` (`|GetArrayItem` (`self.Targets`))) :`TraceChannel` "TraceTypeQuery1" :`DrawDebugType` "ForDuration"))
    (if (`self.ActorHasTag` (`.HitActor` (`GameplayStatics.BreakHitResult` _outhit)) (`self.EnemyTag`))
      (`|ExecutionSequence`
        (:`then_0`
          ;[1 1 1] Base Rotation
          (bind (_direction _newtrack_0) (`Timeline|Timeline_0` :!via `PlayFromStart` :!label _label)
            (:`Update`
              (if (> (`KismetArrayLibrary.Array_Length` _targets_2) 0)
                (bind (_returnvalue_roll _returnvalue_pitch _returnvalue_yaw) (`KismetMathLibrary.BreakRotator` (`KismetMathLibrary.RLerp` (`SceneComponent.K2_GetComponentRotation` _base) (`KismetMathLibrary.FindLookAtRotation` (`SceneComponent.K2_GetComponentLocation` _base) (`self.K2_GetActorLocation` (`|GetArrayItem` _targets_2))) _newtrack_0 true)))
                (`SceneComponent.K2_SetWorldRotation` (`self.Base`) (`KismetMathLibrary.MakeRotator` 0.0 0.0 _returnvalue_yaw) false false)
                ;[1 1 1] Gun Rotation
                (bind (_direction_2 _newtrack_0_2) (`Timeline|Timeline_1` :!via `PlayFromStart` :!label _label_2)
                  (:`Update`
                    (if (> (`KismetArrayLibrary.Array_Length` _targets) 0)
                      (bind (_returnvalue_roll_2 _returnvalue_pitch_2) (`KismetMathLibrary.BreakRotator` (`KismetMathLibrary.RLerp` (`SceneComponent.K2_GetComponentRotation` _gun) (`KismetMathLibrary.FindLookAtRotation` (`SceneComponent.K2_GetComponentLocation` _gun) (`self.K2_GetActorLocation` (`|GetArrayItem` _targets))) _newtrack_0_2 true)))
                      (`SceneComponent.K2_SetWorldRotation` (`self.Gun`) (`KismetMathLibrary.MakeRotator` 0.0 (`KismetMathLibrary.FClamp` _returnvalue_pitch_2 -20.0) _returnvalue_yaw) false false)
                      ;[1 1 1] Shooting
                      (set `self.Shoot Time` (+ (`GameplayStatics.GetWorldDeltaSeconds`) (`self.Shoot Time`)))
                      (if (>= (`self.Shoot Time`) (`self.Fire Rate`))
                        (bind _returnvalue (`|SpawnActorFromClass` "/Game/Blueprints/Old/BP_TestProjectile.BP_TestProjectile_C" (`KismetMathLibrary.MakeTransform` (+ _returnvalue_location (+ (`KismetMathLibrary.GetForwardVector` _returnvalue_rotation) 10.0)) _returnvalue_rotation) "Undefined" "OverrideRootScale" null null))
                        (`|ExecutionSequence`
                          (:`then_0`
                            (set `/Game/Blueprints/Old/BP_TestProjectile.WeaponType` (`self.WeaponType`) _returnvalue))
                          (:`then_1`
                            (set `/Game/Blueprints/Old/BP_TestProjectile.Damage` (`self.Damage`) _returnvalue))
                          (:`then_2`
                            (set `/Game/Blueprints/Old/BP_TestProjectile.DamagePerc` (`self.DamagePerc`) _returnvalue))
                          (:`then_3`
                            (set `/Game/Blueprints/Old/BP_TestProjectile.PiercingPerc` (`self.PiercingPerc`) _returnvalue))
                          (:`then_4`
                            (set `/Game/Blueprints/Old/BP_TestProjectile.ShieldPerc` (`self.ShieldPerc`) _returnvalue))
                          (:`then_5`
                            (set `/Game/Blueprints/Old/BP_TestProjectile.ElementPierc` 0.0 _returnvalue))
                          (:`then_6`
                            (set `self.Shoot Time` 0.0))))
                      (else
                        (goto _label_2 :!via `Stop`)))))
                (else
                  (goto _label :!via `Stop`))))))))))

(fn `RemoveFromArray`
  (params (ActorToRemove :type "Actor Object Reference"))
  (locals (Actor :type "Actor Object Reference"))
  (set `local.Actor` ActorToRemove)
  (if (> (`KismetArrayLibrary.Array_Length` (`self.Targets`)) 0)
    (if (`KismetArrayLibrary.Array_Contains` (`self.Targets`) (`local.Actor`))
      (for (_array_element _array_index) (`self.Targets`)
        (if (== _array_element (`local.Actor`))
          (`KismetArrayLibrary.Array_Remove` (`self.Targets`) _array_index)))
      (if (== (`KismetArrayLibrary.Array_Length` (`self.Targets`)) 0)
        (set `self.Enemy Is Near` false)))))

(fn `SortArray`
  (locals (EnemyGround :type "Array of Actor Object Reference") (EnemyGroundHeavy :type "Array of Actor Object Reference") (EnemyAir :type "Array of Actor Object Reference") (EnemyAirHeavy :type "Array of Actor Object Reference"))
  (switch `/Game/Enums/EWeaponType` (`self.WeaponType`)
    (:`NewEnumerator0`
      (for _array_element (`self.Targets`)
        (if (`self.ActorHasTag` _array_element "Enemy_GroundHeavy")
          (`KismetArrayLibrary.Array_Add` (`local.EnemyGroundHeavy`) _array_element)
          (elif (`self.ActorHasTag` _array_element "Enemy_Ground")
            (`KismetArrayLibrary.Array_Add` (`local.EnemyGround`) _array_element))))
      (if (> (`KismetArrayLibrary.Array_Length` (`local.EnemyGround`)) 0)
        (if (> (`KismetArrayLibrary.Array_Length` (`local.EnemyGroundHeavy`)) 0)
          (`KismetArrayLibrary.Array_Clear` (`self.Targets`))
          (for _array_element_2 (`local.EnemyGroundHeavy`)
            (`KismetArrayLibrary.Array_Add` (`self.Targets`) _array_element_2))
          (`KismetArrayLibrary.Array_Clear` (`local.EnemyGroundHeavy`))
          (for _array_element_3 (`local.EnemyGround`)
            (`KismetArrayLibrary.Array_Add` (`self.Targets`) _array_element_3))
          (`KismetArrayLibrary.Array_Clear` (`local.EnemyGround`)))))
    (:`NewEnumerator1`
      (for _array_element_4 (`self.Targets`)
        (if (`self.ActorHasTag` _array_element_4 "Enemy_Ground")
          (`KismetArrayLibrary.Array_Add` (`local.EnemyGround`) _array_element_4)
          (elif (`self.ActorHasTag` _array_element_4 "Enemy_GroundHeavy")
            (`KismetArrayLibrary.Array_Add` (`local.EnemyGroundHeavy`) _array_element_4))))
      (if (> (`KismetArrayLibrary.Array_Length` (`local.EnemyGroundHeavy`)) 0)
        (if (> (`KismetArrayLibrary.Array_Length` (`local.EnemyGround`)) 0)
          (`KismetArrayLibrary.Array_Clear` (`self.Targets`))
          (for _array_element_5 (`local.EnemyGround`)
            (`KismetArrayLibrary.Array_Add` (`self.Targets`) _array_element_5))
          (`KismetArrayLibrary.Array_Clear` (`local.EnemyGround`))
          (for _array_element_6 (`local.EnemyGroundHeavy`)
            (`KismetArrayLibrary.Array_Add` (`self.Targets`) _array_element_6))
          (`KismetArrayLibrary.Array_Clear` (`local.EnemyGroundHeavy`)))))))

(fn `UpdateTower`
  (params (State :type Integer))
  (switch `int` State
    (:`0`
      (set `self.Fire Rate` (- (`self.Fire Rate`) 0.5)))
    (:`1`
      (set `self.Fire Rate` (- (`self.Fire Rate`) 0.5)))
    (:`2`
      (set `self.Fire Rate` (- (`self.Fire Rate`) 0.5)))))

(fn `UserConstructionScript`
  (bind _collision (`self.Collision`))
  (bind (_returnvalue_x _returnvalue_y _returnvalue_z) (`KismetMathLibrary.BreakVector` (`SceneComponent.K2_GetComponentScale` _collision)))
  (bind _returnvalue (+ _returnvalue_x (`KismetMathLibrary.Conv_IntToDouble` (`self.Range`))))
  (`SceneComponent.SetWorldScale3D` _collision (`KismetMathLibrary.MakeVector` _returnvalue _returnvalue _returnvalue_z)))