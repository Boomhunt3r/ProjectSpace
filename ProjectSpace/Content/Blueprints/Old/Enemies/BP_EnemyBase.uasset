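; Base tower-defense enemy that walks to a destination, damaging the player by its Strength on arrival.
; Tagged projectiles feed GetDamage, which splits hits between Shield and piercing Health damage until the shield drops, then applies full-damage percentage to Health.
; A broken shield retags heavy ground enemies and removes them from heavy ground towers' target arrays.
; On death or arrival it deregisters from all towers and its spawner, then destroys itself.
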(event `self.ReceiveBeginPlay`
  (bind _outactors (`GameplayStatics.GetAllActorsOfClass` "/Game/Blueprints/Old/Tower/BP_Tower.BP_Tower_C"))
  (set `self.Towers` _outactors)
  (bind _asui_enemy_health (cast `/Game/Blueprints/Old/Enemies/UI_Enemy_Health` (`WidgetComponent.GetUserWidgetObject` (`self.Widget`))))
  (`/Game/Blueprints/Old/Enemies/UI_Enemy_Health.Unique Owner` _asui_enemy_health self)
  (bind _astop_down_character (cast `/Game/TopDownBP/Blueprints/TopDownCharacter` (`GameplayStatics.GetPlayerCharacter` 0)))
  (set `self.PlayerRef` _astop_down_character))

(event `self.ReceiveActorBeginOverlap`
  (params (OtherActor :type "Actor Object Reference"))
  ;[1 1 1] Enemy hit logic
  (if (`self.ActorHasTag` OtherActor "Projectile")
    (bind _asbp_test_projectile (cast `/Game/Blueprints/Old/BP_TestProjectile` OtherActor))
    (bind _output_get (set `self.Bullet` _asbp_test_projectile))
    (`self.GetDamage` (`/Game/Blueprints/Old/BP_TestProjectile.Damage` _output_get) (`/Game/Blueprints/Old/BP_TestProjectile.ShieldPerc` _output_get) (`/Game/Blueprints/Old/BP_TestProjectile.PiercingPerc` _output_get) (`/Game/Blueprints/Old/BP_TestProjectile.DamagePerc` _output_get) (`/Game/Blueprints/Old/BP_TestProjectile.WeaponType` _output_get))
    (`self.K2_DestroyActor` _output_get)))

(event `self.ReceiveTick`
  (params (DeltaSeconds :type "Float (single-precision)"))
  (if (<= (`self.Health`) 0.0)
    (for _array_element (`self.Towers`)
      (bind _asbp_tower (cast `/Game/Blueprints/Old/Tower/BP_Tower` _array_element))
      (`/Game/Blueprints/Old/Tower/BP_Tower.RemoveFromArray` _asbp_tower self))
    (`/Game/Blueprints/Old/EnemySpawner/BP_EnemySpawner.RemoveEnemyFromArray` (`self.Spawner`) self)
    (`self.K2_DestroyActor`)
    (else
      (`|AIMoveTo` (`PawnMovementComponent.GetPawnOwner` (`self.CharacterMovement`)) (`self.K2_GetActorLocation` (`self.Destination`)) null
        (:`OnSuccess`
          (for _array_element_2 (`self.Towers`)
            (bind _asbp_tower_2 (cast `/Game/Blueprints/Old/Tower/BP_Tower` _array_element_2))
            (`/Game/Blueprints/Old/Tower/BP_Tower.RemoveFromArray` _asbp_tower_2 self))
          (`/Game/TopDownBP/Blueprints/TopDownCharacter.DecreaseHealth` (`self.PlayerRef`) (`self.Strength`))
          (`/Game/Blueprints/Old/EnemySpawner/BP_EnemySpawner.RemoveEnemyFromArray` (`self.Spawner`) self)
          (`self.K2_DestroyActor`))))))

(fn `GetDamage`
  (params (Damage :type "Float (double-precision)") (ShieldPerc :type "Float (double-precision)") (PiercPerc :type "Float (double-precision)") (DamagePerc :type "Float (double-precision)") (WeaponType :type "/Game/Enums/EWeaponType Enum" :default "NewEnumerator0"))
  (locals (`Weapon Type` :type "/Game/Enums/EWeaponType Enum") (IncomingDamge :type "Float (double-precision)") (IncomingShieldPerc :type "Float (double-precision)") (IncomingPiercPerc :type "Float (double-precision)") (IncomingDamagePerc :type "Float (double-precision)"))
  (set `local.IncomingDamge` Damage)
  (set `local.IncomingShieldPerc` ShieldPerc)
  (set `local.IncomingPiercPerc` PiercPerc)
  (set `local.IncomingDamagePerc` DamagePerc)
  (set `local.Weapon Type` WeaponType)
  (if (> (`self.Shield`) 0.0)
    (switch `/Game/Enums/EWeaponType` (`local.Weapon Type`)
      (:`NewEnumerator0`
        (set `self.Shield` (- (`self.Shield`) (* (`local.IncomingDamge`) (`local.IncomingShieldPerc`))))
        (set `self.Health` (- (`self.Health`) (* (`local.IncomingDamge`) (`local.IncomingPiercPerc`)))))
      (:`NewEnumerator1`
        (set `self.Shield` (- (`self.Shield`) (* (`local.IncomingDamge`) (`local.IncomingShieldPerc`))))
        (set `self.Health` (- (`self.Health`) (* (`local.IncomingDamge`) (`local.IncomingPiercPerc`)))))
      (:`NewEnumerator2`
        (set `self.Shield` (- (`self.Shield`) (* (`local.IncomingDamge`) (`local.IncomingShieldPerc`))))
        (set `self.Health` (- (`self.Health`) (* (`local.IncomingDamge`) (`local.IncomingPiercPerc`)))))
      (:`NewEnumerator3`
        (set `self.Shield` (- (`self.Shield`) (* (`local.IncomingDamge`) (`local.IncomingShieldPerc`))))
        (set `self.Health` (- (`self.Health`) (* (`local.IncomingDamge`) (`local.IncomingPiercPerc`))))))
    (if (<= (`self.Shield`) 0.0)
      (set `self.shield down` true)
      (switch `/Game/Enums/EEnemyType` (`self.EnemyType`)
        (:`NewEnumerator1`
          (set `self.Tags` (`|MakeArray` "Enemy_Ground" :!type "Name"))
          (for _array_element (`self.Towers`)
            (if (`self.ActorHasTag` _array_element "Tower_GroundHeavy")
              (bind _asbpc_tower_heavy (cast `/Game/Blueprints/Old/Tower/BPC_Tower_Heavy` _array_element))
              (`/Game/Blueprints/Old/Tower/BP_Tower.RemoveFromArray` _asbpc_tower_heavy self))))))
    (else
      (set `self.shield down` true)
      (if (<= (`self.Shield`) 0.0)
        (switch `/Game/Enums/EWeaponType` (`local.Weapon Type`)
          (:`NewEnumerator0`
            (set `self.Health` (- (`self.Health`) (* (`local.IncomingDamge`) (`local.IncomingDamagePerc`)))))
          (:`NewEnumerator1`
            (set `self.Health` (- (`self.Health`) (* (`local.IncomingDamge`) (`local.IncomingDamagePerc`)))))
          (:`NewEnumerator2`
            (set `self.Health` (- (`self.Health`) (* (`local.IncomingDamge`) (`local.IncomingDamagePerc`)))))
          (:`NewEnumerator3`
            (set `self.Health` (- (`self.Health`) (* (`local.IncomingDamge`) (`local.IncomingDamagePerc`))))))))))

(fn `UserConstructionScript`)