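; BP_EnemyGround is a ground enemy that moves toward a stored Location and takes damage from projectiles.
; BeginPlay caches actors tagged Tower_Ground and passes itself to its health widget.
; Overlapping projectiles subtract their Damage from Health and are destroyed.
; Tick prints Health and issues the move, or at zero Health calls RemoveFromArray on each cached tower and destroys the enemy.
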(event `self.ReceiveBeginPlay`
  (bind _outactors (`GameplayStatics.GetAllActorsWithTag` "Tower_Ground"))
  (set `self.Towers` _outactors)
  (bind _asui_enemy_health (cast `/Game/Blueprints/Ground_Enemy/UI_Enemy_Health` (`WidgetComponent.GetUserWidgetObject` (`self.Widget`))))
  (`/Game/Blueprints/Ground_Enemy/UI_Enemy_Health.Unique Owner` _asui_enemy_health self))

(event `self.ReceiveActorBeginOverlap`
  (params (OtherActor :type "Actor Object Reference"))
  ;[1 1 1] Enemy hit logic
  (if (`self.ActorHasTag` OtherActor "Projectile")
    (bind _asbp_test_projectile (cast `/Game/Blueprints/BP_TestProjectile` OtherActor))
    (bind _output_get (set `self.Bullet` _asbp_test_projectile))
    (`self.GetDamage` (`/Game/Blueprints/BP_TestProjectile.Damage` _output_get))
    (`self.K2_DestroyActor` _output_get)))

(event `self.ReceiveTick`
  (params (DeltaSeconds :type "Float (single-precision)"))
  (`KismetSystemLibrary.PrintString` (`KismetStringLibrary.Conv_IntToString` (`self.Health`)))
  (if (<= (`self.Health`) 0)
    (for _array_element (`self.Towers`)
      (bind _asbp_tower (cast `/Game/Blueprints/Tower/BP_Tower` _array_element))
      (`/Game/Blueprints/Tower/BP_Tower.RemoveFromArray` _asbp_tower))
    (`self.K2_DestroyActor`)
    (else
      (`AIBlueprintHelperLibrary.SimpleMoveToLocation` (`self.GetController`) (`self.Location`)))))

(fn `GetDamage`
  (params (Damage :type Integer))
  (set `self.Health` (- (`self.Health`) Damage)))

(fn `UserConstructionScript`)