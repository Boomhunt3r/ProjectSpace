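; Defense tower actor that automatically tracks and shoots enemies inside a collision area widened by its Range.
; Overlap events keep a list of actors with the enemy tag, and Tick turns the base and pitch-clamped gun toward the first entry.
; A delta-time timer spawns BP_TestProjectile at the FireRate interval, passing on weapon and damage stats.
; UpdateTower shortens that interval by the same step for each handled state.
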(event `self.ReceiveBeginPlay`
  (`SceneComponent.SetVisibility` (`self.Collision`) false false))

(event `self.ReceiveActorBeginOverlap`
  (params (OtherActor :type "Actor Object Reference"))
  ;[1 1 1] Is Enemy in Range?
  (if (`self.ActorHasTag` OtherActor (`self.EnemyTag`))
    (set `self.Enemy Is Near` true)
    (bind _output_get (set `self.Target` OtherActor))
    (`KismetArrayLibrary.Array_Add` (`self.Targets`) _output_get)))

(event `self.ReceiveActorEndOverlap`
  (params (OtherActor :type "Actor Object Reference"))
  ;[1 1 1] Is Enemy in Range?
  (if (`self.ActorHasTag` OtherActor (`self.EnemyTag`))
    (`self.RemoveFromArray` OtherActor)
    (if (== (`KismetArrayLibrary.Array_Length` (`self.Targets`)) 0)
      (set `self.Enemy Is Near` false))))

(event `self.ReceiveTick`
  (params (DeltaSeconds :type "Float (single-precision)"))
  (bind (_returnvalue_location _returnvalue_rotation) (`KismetMathLibrary.BreakTransform` (`SceneComponent.K2_GetComponentToWorld` (`self.Gun`))))
  (bind _returnvalue (`self.K2_GetActorLocation` (`|GetArrayItem` (`self.Targets`))))
  (bind (_returnvalue_roll _returnvalue_pitch) (`KismetMathLibrary.BreakRotator` (`KismetMathLibrary.FindLookAtRotation` (`SceneComponent.K2_GetComponentLocation` (`self.Gun`)) _returnvalue)))
  (bind (_returnvalue_roll_2 _returnvalue_pitch_2 _returnvalue_yaw) (`KismetMathLibrary.BreakRotator` (`KismetMathLibrary.FindLookAtRotation` (`SceneComponent.K2_GetComponentLocation` (`self.Base`)) _returnvalue)))
  (if (> (`KismetArrayLibrary.Array_Length` (`self.Targets`)) 0)
    (if (`self.Enemy Is Near`)
      (`SceneComponent.K2_SetWorldRotation` (`self.Base`) (`KismetMathLibrary.MakeRotator` 0.0 0.0 _returnvalue_yaw) false false)
      (`SceneComponent.K2_SetWorldRotation` (`self.Gun`) (`KismetMathLibrary.MakeRotator` _returnvalue_roll_2 (`KismetMathLibrary.FClamp` _returnvalue_pitch -20.0) _returnvalue_yaw) false false)
      (set `self.Shoot Time` (+ (`GameplayStatics.GetWorldDeltaSeconds`) (`self.Shoot Time`)))
      (if (>= (`self.Shoot Time`) (`self.Fire Rate`))
        (bind _returnvalue_2 (`|SpawnActorFromClass` "/Game/Blueprints/BP_TestProjectile.BP_TestProjectile_C" (`KismetMathLibrary.MakeTransform` (+ _returnvalue_location (+ (`KismetMathLibrary.GetForwardVector` _returnvalue_rotation) 10.0)) _returnvalue_rotation) "Undefined" "OverrideRootScale" null null))
        (`|ExecutionSequence`
          (:`then_0`
            (set `/Game/Blueprints/BP_TestProjectile.WeaponType` (`self.WeaponType`) _returnvalue_2))
          (:`then_1`
            (set `/Game/Blueprints/BP_TestProjectile.Damage` (`self.Damage`) _returnvalue_2))
          (:`then_2`
            (set `/Game/Blueprints/BP_TestProjectile.DamagePerc` (`self.DamagePerc`) _returnvalue_2))
          (:`then_3`
            (set `/Game/Blueprints/BP_TestProjectile.PiercingPerc` (`self.PiercingPerc`) _returnvalue_2))
          (:`then_4`
            (set `/Game/Blueprints/BP_TestProjectile.ShieldPerc` (`self.ShieldPerc`) _returnvalue_2))
          (:`then_5`
            (set `/Game/Blueprints/BP_TestProjectile.ElementPierc` 0.0 _returnvalue_2))
          (:`then_6`
            (set `self.Shoot Time` 0.0)))))))

(fn `RemoveFromArray`
  (params (ActorToRemove :type "Actor Object Reference"))
  (locals (Actor :type "Actor Object Reference"))
  (set `local.Actor` ActorToRemove)
  (if (> (`KismetArrayLibrary.Array_Length` (`self.Targets`)) 0)
    (if (`KismetArrayLibrary.Array_Contains` (`self.Targets`) (`local.Actor`))
      (for (_array_element _array_index) (`self.Targets`)
        (if (== _array_element (`local.Actor`))
          (`KismetArrayLibrary.Array_Remove` (`self.Targets`) _array_index))))))

(fn `UpdateTower`
  (params (State :type Integer))
  (switch `int` State
    (:`0`
      (set `self.Fire Rate` (- (`self.Fire Rate`) 0.5)))
    (:`1`
      (set `self.Fire Rate` (- (`self.Fire Rate`) 0.5)))
    (:`2`
      (set `self.Fire Rate` (- (`self.Fire Rate`) 0.5)))))

(fn `UserConstructionScript`
  (bind _collision (`self.Collision`))
  (bind (_returnvalue_x _returnvalue_y _returnvalue_z) (`KismetMathLibrary.BreakVector` (`SceneComponent.K2_GetComponentScale` _collision)))
  (bind _returnvalue (+ _returnvalue_x (`KismetMathLibrary.Conv_IntToDouble` (`self.Range`))))
  (`SceneComponent.SetWorldScale3D` _collision (`KismetMathLibrary.MakeVector` _returnvalue _returnvalue _returnvalue_z)))