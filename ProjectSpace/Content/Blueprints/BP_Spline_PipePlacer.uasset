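; Spline-driven placer that builds pipe runs from spline mesh components in the Construction Script when SpawnMeshes is on.
; It divides the spline by SectionLength, with FitInLastMesh adjusting the count, and bends each segment using scaled direction tangents.
; Optional start and end meshes sit at the first and last spline points with their own axis, scale and material.
; All pieces share collision, mobility and visibility settings.
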(fn `UserConstructionScript`
  (locals (`Spline Length` :type Integer :default 0))
  (bind _spline (`self.Spline`))
  (bind _spline_2 (`self.Spline`))
  (bind _spline_3 (`self.Spline`))
  (bind _returnvalue (- (`SplineComponent.GetNumberOfSplinePoints` (`self.Spline`)) 1))
  (bind _returnvalue_2 (`KismetMathLibrary.FTrunc` (/ (`SplineComponent.GetSplineLength` (`self.Spline`)) (`self.Section Length`))))
  (if (`self.Spawn Meshes`)
    (if (`self.Specific Start/End Mesh?`)
      (`|ExecutionSequence`
        (:`then_0`
          ;[1 1 1] start Mesh
          (bind _returnvalue_3 (`AddComponent|NODE_AddSplineMeshComponent-1` :`RelativeTransform` (`KismetMathLibrary.MakeTransform` (0.0 0.0 0.0) (struct) (1.0 1.0 1.0))))
          (`StaticMeshComponent.SetStaticMesh` _returnvalue_3 (`self.Mesh_Start`))
          (`SplineMeshComponent.SetForwardAxis` _returnvalue_3 (`self.Forward Axis_Start`) true)
          (`SceneComponent.K2_SetWorldLocationAndRotation` _returnvalue_3 (`SplineComponent.GetLocationAtSplinePoint` _spline_2 0 "World") (`SplineComponent.GetRotationAtSplinePoint` _spline_2 0 "World") false false)
          (`SceneComponent.SetRelativeScale3D` _returnvalue_3 (`self.Scale_Start`))
          (`PrimitiveComponent.SetMaterial` _returnvalue_3 0 (`self.Material_Start`))
          (`PrimitiveComponent.SetCollisionEnabled` _returnvalue_3 (`self.Collision`) :!label _label)
          (`PrimitiveComponent.SetCollisionEnabled` (stale _returnvalue_4) (`self.Collision`))
          (`PrimitiveComponent.SetCollisionEnabled` (stale _returnvalue_5) (`self.Collision`))
          (`SceneComponent.SetMobility` _returnvalue_3 (`self.Mobility`))
          (`SceneComponent.SetMobility` (stale _returnvalue_4) (`self.Mobility`))
          (`SceneComponent.SetMobility` (stale _returnvalue_5) (`self.Mobility`))
          (`SceneComponent.SetVisibility` _returnvalue_3 (`self.Visibility`) false)
          (`SceneComponent.SetVisibility` (stale _returnvalue_4) (`self.Visibility`) false)
          (`SceneComponent.SetVisibility` (stale _returnvalue_5) (`self.Visibility`) false))
        (:`then_1`
          ;[1 1 1] End Mesh
          (bind _returnvalue_4 (`AddComponent|NODE_AddSplineMeshComponent-2`))
          (`StaticMeshComponent.SetStaticMesh` _returnvalue_4 (`self.Mesh_End`))
          (`SplineMeshComponent.SetForwardAxis` _returnvalue_4 (`self.Forward Axis_End`) true)
          (`SceneComponent.K2_SetWorldLocationAndRotation` _returnvalue_4 (`SplineComponent.GetLocationAtSplinePoint` _spline_3 _returnvalue "World") (`SplineComponent.GetRotationAtSplinePoint` _spline_3 _returnvalue "World") false false)
          (`SceneComponent.SetRelativeScale3D` _returnvalue_4 (`self.Scale_End`))
          (`PrimitiveComponent.SetMaterial` _returnvalue_4 0 (`self.Material_End`))
          (goto _label))
        (:`then_2`
          (if (`self.Fit in Last Mesh`) :!label _label_2
            (set `local.Spline Length` _returnvalue_2)
            (else
              (bind _result (`/Engine/EditorBlueprintResources/StandardMacros.DecrementInt` _returnvalue_2)
                (:`  `
                  (set `local.Spline Length` _result)))))
          (for _index (range (+ (`local.Spline Length`) 1))
            (bind _returnvalue_5 (`AddComponent|NODE_AddSplineMeshComponent-0`))
            (`StaticMeshComponent.SetStaticMesh` _returnvalue_5 (`self.StaticMesh`))
            (`SplineMeshComponent.SetForwardAxis` _returnvalue_5 (`self.Forward Axis `) true)
            (`PrimitiveComponent.SetMaterial` _returnvalue_5 0 (`self.Material`))
            (bind _returnvalue_6 (* _index (`self.Section Length`)))
            (bind _returnvalue_7 (* (+ _index 1) (`self.Section Length`)))
            (`SplineMeshComponent.SetStartAndEnd` _returnvalue_5 (`SplineComponent.GetLocationAtDistanceAlongSpline` _spline _returnvalue_6 "Local") (* (`SplineComponent.GetDirectionAtDistanceAlongSpline` _spline _returnvalue_6 "Local") (`self.Tangent`)) (`SplineComponent.GetLocationAtDistanceAlongSpline` _spline _returnvalue_7 "Local") (* (`SplineComponent.GetDirectionAtDistanceAlongSpline` _spline _returnvalue_7 "Local") (`self.Tangent`)) true)
            (goto _label))))
      (else
        (goto _label_2)))))