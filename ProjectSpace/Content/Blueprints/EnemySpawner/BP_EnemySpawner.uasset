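; BP_EnemySpawner spawns a limited number of BP_EnemyGround AI enemies at its root's world location.
; While CanSpawn is set, Tick accumulates delta time and spawns an enemy each time the timer reaches SpawnTime.
; The timer reset and spawn count follow only a successful cast of the spawned pawn, and CanSpawn clears once the count reaches AmountToSpawn.
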(event `self.ReceiveTick`
  (params (DeltaSeconds :type "Float (single-precision)"))
  (bind _totalspawned (`self.TotalSpawned`))
  (if (`self.CanSpawn`)
    (set `self.SpawnTimer` (+ DeltaSeconds (`self.SpawnTimer`)))
    (if (>= (`self.SpawnTimer`) (`self.SpawnTime`))
      (bind _returnvalue (`AIBlueprintHelperLibrary.SpawnAIFromClass` "/Game/Blueprints/Ground_Enemy/BP_EnemyGround.BP_EnemyGround_C" null (`SceneComponent.K2_GetComponentLocation` (`self.DefaultSceneRoot`)) (struct) false null))
      (cast `/Game/Blueprints/Ground_Enemy/BP_EnemyGround` _returnvalue)
      (set `self.SpawnTimer` 0.0)
      (`/Engine/EditorBlueprintResources/StandardMacros.IncrementInt` _totalspawned
        (:`  `
          (if (>= _totalspawned (`self.AmountToSpawn`))
            (set `self.CanSpawn` false)))))))

(fn `UserConstructionScript`)