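; Spline actor that lays track indicator decals as an editor-time guide and hides its component hierarchy on BeginPlay.
; The Construction Script first snaps spline points onto surfaces found by line traces within a SnappingThreshold offset either side of each point.
; It then adds decals at DecalSpacing intervals along the snapped spline, projected downward, rotated to follow its direction and sized by DecalScale.
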(event `self.ReceiveBeginPlay`
  (`SceneComponent.SetVisibility` (`self.DefaultSceneRoot`) false true))

(fn `UserConstructionScript`
  (bind _spline (`self.Spline`))
  (bind _decal_scale (`self.Decal Scale`))
  (`|ExecutionSequence`
    (:`then_0`
      (bind _result (`/Engine/EditorBlueprintResources/StandardMacros.DecrementInt` (`SplineComponent.GetNumberOfSplinePoints` (`self.Spline`)))
        (:`  `
          (for _index (range (+ _result 1))
            (bind (_outhit _returnvalue) (`KismetSystemLibrary.LineTraceSingle` (+ (`SplineComponent.GetLocationAtSplinePoint` (`self.Spline`) _index "World") (`self.Snapping Threshold`)) (- (`SplineComponent.GetLocationAtSplinePoint` (`self.Spline`) _index "World") (`self.Snapping Threshold`)) "TraceTypeQuery1"))
            (if _returnvalue
              (`SplineComponent.SetLocationAtSplinePoint` (`self.Spline`) _index (`.Location` (`GameplayStatics.BreakHitResult` _outhit)) "World" true))))))
    (:`then_1`
      (for _index_2 (range (+ (`KismetMathLibrary.FTrunc` (/ (`SplineComponent.GetSplineLength` (`self.Spline`)) (`self.Decal Spacing`))) 1))
        (bind _returnvalue_2 (`AddComponent|NODE_AddDecalComponent-0` :`RelativeTransform` (`KismetMathLibrary.MakeTransform` (0.0 0.0 0.0) (struct :`Yaw` 90.0))))
        (bind _returnvalue_3 (* _index_2 (`self.Decal Spacing`)))
        (bind (_returnvalue_roll _returnvalue_pitch _returnvalue_yaw) (`KismetMathLibrary.BreakRotator` (`SplineComponent.GetRotationAtDistanceAlongSpline` _spline _returnvalue_3 "Local")))
        (`SceneComponent.K2_SetWorldTransform` _returnvalue_2 (`KismetMathLibrary.MakeTransform` (`SplineComponent.GetLocationAtDistanceAlongSpline` _spline _returnvalue_3 "World") (`KismetMathLibrary.MakeRotator` (- _returnvalue_roll 90.0) 90.0 _returnvalue_yaw) (`KismetMathLibrary.MakeVector` _decal_scale _decal_scale _decal_scale)) false false)
        (`DecalComponent.SetDecalMaterial` _returnvalue_2 "/Game/Materials/Master/M_Decal_TrackIndicator.M_Decal_TrackIndicator")))))