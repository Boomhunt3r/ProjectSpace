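; BP_Tower is an auto-firing turret that activates when an actor tagged Enemy_Ground overlaps it.
; Overlap events set EnemyIsNear, though any untagged actor ending overlap also sets it true.
; While the flag is set, Tick rotates TurretFrame toward player character 0, not the detected enemy, with clamped pitch.
; A delta-time accumulator spawns BP_TestProjectile near TurretBarrel at each FireRate interval, and Tick also prints the flag for debugging.
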(event `self.ReceiveActorBeginOverlap`
  (params (OtherActor :type "Actor Object Reference"))
  ;[1 1 1] Is Enemy in Range?
  (set `self.Enemy Is Near` (`self.ActorHasTag` OtherActor "Enemy_Ground")))

(event `self.ReceiveActorEndOverlap`
  (params (OtherActor :type "Actor Object Reference"))
  ;[1 1 1] Is Enemy in Range?
  (set `self.Enemy Is Near` (not (`self.ActorHasTag` OtherActor "Enemy_Ground"))))

(event `self.ReceiveTick`
  (params (DeltaSeconds :type "Float (single-precision)"))
  (bind _turret_frame (`self.Turret_Frame`))
  (bind (_returnvalue_location _returnvalue_rotation) (`KismetMathLibrary.BreakTransform` (`SceneComponent.K2_GetComponentToWorld` (`self.Turret_Barrel`))))
  (bind (_returnvalue_roll _returnvalue_pitch _returnvalue_yaw) (`KismetMathLibrary.BreakRotator` (`KismetMathLibrary.FindLookAtRotation` (`SceneComponent.K2_GetComponentLocation` _turret_frame) (`self.K2_GetActorLocation` (`GameplayStatics.GetPlayerCharacter` 0)))))
  (`KismetSystemLibrary.PrintString` (`KismetStringLibrary.Conv_BoolToString` (`self.Enemy Is Near`)))
  (if (`self.Enemy Is Near`)
    (`SceneComponent.K2_SetWorldRotation` _turret_frame (`KismetMathLibrary.MakeRotator` _returnvalue_roll (`KismetMathLibrary.FClamp` _returnvalue_pitch -10.0) _returnvalue_yaw) false false)
    (set `self.Shoot Time` (+ (`GameplayStatics.GetWorldDeltaSeconds`) (`self.Shoot Time`)))
    (if (>= (`self.Shoot Time`) (`self.Fire Rate`))
      (`|SpawnActorFromClass` "/Game/Blueprints/BP_TestProjectile.BP_TestProjectile_C" (`KismetMathLibrary.MakeTransform` (+ _returnvalue_location (+ (`KismetMathLibrary.GetForwardVector` _returnvalue_rotation) 10.0)) _returnvalue_rotation) "Undefined" "OverrideRootScale" null null)
      (set `self.Shoot Time` 0.0))))

(fn `UserConstructionScript`)