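; Storage actor that steps four boards downward and starts a round when a tagged cube reaches its start trigger.
; A cube entering the move trigger lowers the boards by a fixed step through a timeline lerp.
; The start trigger, guarded by RoundRunning, starts the cube and makes every BP_TowerBase follow it.
; Teleport_Board relocates a board whose target nears the bottom position, but nothing here calls it.
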(event `Move_Storage`
  (bind _board_02 (`self.Board_02`))
  (bind _board_03 (`self.Board_03`))
  (bind _board_04 (`self.Board_04`))
  (bind _board_01 (`self.Board_01`))
  ;[1 1 1] Move Storage
  (set `self.Board_01_update` (- (`SceneComponent.RelativeLocation` (`self.Board_01`)) (0.0 0.0 130.0)))
  (set `self.Board_02_Update` (- (`SceneComponent.RelativeLocation` (`self.Board_02`)) (0.0 0.0 130.0)))
  (set `self.Board_03_Update` (- (`SceneComponent.RelativeLocation` (`self.Board_03`)) (0.0 0.0 130.0)))
  (set `self.Board_04_Update` (- (`SceneComponent.RelativeLocation` (`self.Board_04`)) (0.0 0.0 130.0)))
  (set `self.Locator_Update` (- (`SceneComponent.RelativeLocation` (`self.TP_Locator`)) (0.0 0.0 130.0)))
  (bind (_direction _0_1) (`Timeline|Lerp 0-1` :!via `PlayFromStart`)
    (:`Update`
      (`|ExecutionSequence`
        (:`then_0`
          (`SceneComponent.K2_SetRelativeLocation` _board_01 (`KismetMathLibrary.VLerp` (`SceneComponent.RelativeLocation` _board_01) (`self.Board_01_update`) _0_1) false false))
        (:`then_1`
          (`SceneComponent.K2_SetRelativeLocation` _board_02 (`KismetMathLibrary.VLerp` (`SceneComponent.RelativeLocation` _board_02) (`self.Board_02_Update`) _0_1) false false))
        (:`then_2`
          (`SceneComponent.K2_SetRelativeLocation` _board_03 (`KismetMathLibrary.VLerp` (`SceneComponent.RelativeLocation` _board_03) (`self.Board_03_Update`) _0_1) false false))
        (:`then_3`
          (`SceneComponent.K2_SetRelativeLocation` _board_04 (`KismetMathLibrary.VLerp` (`SceneComponent.RelativeLocation` _board_04) (`self.Board_04_Update`) _0_1) false false))))))

(event `self.ReceiveBeginPlay`
  (bind _outactors (`GameplayStatics.GetAllActorsOfClass` "/Game/Blueprints/New/Blueprints/Tower/BP_TowerBase.BP_TowerBase_C"))
  (set `self.Tower Ref` _outactors))

(event `Teleport_Board`
  (bind _teleport_board_to (`self.Teleport Board to`))
  ;[1 1 1] Move Storage
  ;;[1 1 1] Check for Teleport
  (if (== (`self.Board_01_update`) (65.0 0.0 -130.0) :`ErrorTolerance` 20.0)
    (`SceneComponent.K2_SetRelativeLocation` (`self.Board_01`) _teleport_board_to false false)
    (elif (== (`self.Board_02_Update`) (65.0 0.0 -130.0) :`ErrorTolerance` 20.0)
      (`SceneComponent.K2_SetRelativeLocation` (`self.Board_02`) _teleport_board_to false false)
      (elif (== (`self.Board_03_Update`) (65.0 0.0 -130.0) :`ErrorTolerance` 20.0)
        (`SceneComponent.K2_SetRelativeLocation` (`self.Board_03`) _teleport_board_to false false)
        (elif (== (`self.Board_04_Update`) (65.0 0.0 -130.0) :`ErrorTolerance` 20.0)
          (`SceneComponent.K2_SetRelativeLocation` (`self.Board_04`) _teleport_board_to false false))))))

(event `Launch Cube`
  (if (`self.ActorHasTag` (stale `self.Trigger_Start Cube.OnComponentBeginOverlap` OtherActor) "Cube") :!label _label
    (if (not (`self.Round running`))
      (set `self.Round running` true)
      (bind _asbp_cube (cast `/Game/Blueprints/New/Blueprints/Cube/BP_Cube` (stale `self.Trigger_Start Cube.OnComponentBeginOverlap` OtherActor)))
      (`/Game/Blueprints/New/Blueprints/Cube/BP_Cube.Start Cube` _asbp_cube)
      (for _array_element (`self.Tower Ref`)
        (set `/Game/Blueprints/New/Blueprints/Tower/BP_TowerBase.should follow Target` true _array_element)
        (set `/Game/Blueprints/New/Blueprints/Tower/BP_TowerBase.Target Ref` _asbp_cube _array_element)))))

(event `self.Trigger_Start Cube.OnComponentBeginOverlap`
  (params (OverlappedComponent :type "PrimitiveComponent Object Reference") (OtherActor :type "Actor Object Reference") (OtherComp :type "PrimitiveComponent Object Reference") (OtherBodyIndex :type Integer) (bFromSweep :type Boolean) (SweepResult :type "HitResult Structure (by ref)"))
  (goto _label))

(event `self.Trigger_MoveStorage.OnComponentBeginOverlap`
  (params (OverlappedComponent :type "PrimitiveComponent Object Reference") (OtherActor :type "Actor Object Reference") (OtherComp :type "PrimitiveComponent Object Reference") (OtherBodyIndex :type Integer) (bFromSweep :type Boolean) (SweepResult :type "HitResult Structure (by ref)"))
  (if (`self.ActorHasTag` OtherActor "Cube")
    (`self.Move_Storage`)))

(fn `UserConstructionScript`)