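; Temple Blueprint with a double gate that opens and closes when an actor tagged "Cube" enters its trigger components.
; Overlapping the OpenGAte component snaps DoorLeft and DoorRight to mirrored yaw rotations to swing them open.
; Overlapping CloseGate resets both doors to zero rotation, instantly and without animation, and prints a debug "Hello" for any overlapping actor.
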(event `self.open GAte.OnComponentBeginOverlap`
  (params (OverlappedComponent :type "PrimitiveComponent Object Reference") (OtherActor :type "Actor Object Reference") (OtherComp :type "PrimitiveComponent Object Reference") (OtherBodyIndex :type Integer) (bFromSweep :type Boolean) (SweepResult :type "HitResult Structure (by ref)"))
  (if (`self.ActorHasTag` OtherActor "Cube")
    (`SceneComponent.K2_SetRelativeRotation` (`self.Door_left`) (struct :`Yaw` 140.0) false false)
    (`SceneComponent.K2_SetRelativeRotation` (`self.Door_right`) (struct :`Yaw` -140.0) false false)))

(event `self.close Gate.OnComponentBeginOverlap`
  (params (OverlappedComponent :type "PrimitiveComponent Object Reference") (OtherActor :type "Actor Object Reference") (OtherComp :type "PrimitiveComponent Object Reference") (OtherBodyIndex :type Integer) (bFromSweep :type Boolean) (SweepResult :type "HitResult Structure (by ref)"))
  (`KismetSystemLibrary.PrintString` "Hello")
  (if (`self.ActorHasTag` OtherActor "Cube")
    (`SceneComponent.K2_SetRelativeRotation` (`self.Door_left`) (struct) false false)
    (`SceneComponent.K2_SetRelativeRotation` :`self` (`self.Door_right`))))

(fn `UserConstructionScript`)