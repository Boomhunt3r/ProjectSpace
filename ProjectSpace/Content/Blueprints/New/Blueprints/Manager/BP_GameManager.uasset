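; BP_GameManager coordinates game over and high score persistence.
; On BeginPlay it caches the player, cube manager and game instance, then reads the high score from the instance's save object.
; A wrong-color EndGame marks the player dead, ends the cube manager's game and swaps the HUD for the game-over UI.
; SaveHighscore writes the score to the save slot; SelectedGamemode is an empty stub.
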(event `self.ReceiveBeginPlay`
  (bind _returnvalue (`GameplayStatics.GetActorOfClass` "/Game/Blueprints/New/Blueprints/Player/BP_Player.BP_Player_C"))
  (set `self.PlayerRef` _returnvalue)
  (bind _returnvalue_2 (`GameplayStatics.GetActorOfClass` "/Game/Blueprints/New/Blueprints/Cube/BP_CubeManager.BP_CubeManager_C"))
  (set `self.CubeManagerRef` _returnvalue_2)
  (bind _asbp_game_instane (cast `/Game/Blueprints/New/Blueprints/BP_GameInstane` (`GameplayStatics.GetGameInstance`)))
  (bind _output_get (set `self.GameInstanceRef` _asbp_game_instane))
  (set `self.Highscore` (`/Game/Blueprints/New/Blueprints/BP_SaveGame.Highscore` (`/Game/Blueprints/New/Blueprints/BP_GameInstane.SaveGameRef` _output_get))))

(event `Selected Gamemode`
  (params (NewParam :type Boolean) (NewParam2 :type Boolean) (NewParam3 :type Boolean)))

(event `End Game`
  (params (WrogColor :type Boolean))
  (bind _playerref (`self.PlayerRef`))
  (if WrogColor
    (set `/Game/Blueprints/New/Blueprints/Player/BP_Player.isAlive` false _playerref)
    (`/Game/Blueprints/New/Blueprints/Cube/BP_CubeManager.EndGame` (`self.CubeManagerRef`))
    (`Widget.SetVisibility` (`/Game/Blueprints/New/Blueprints/Player/BP_Player.UI_HUD` _playerref) "Hidden")
    (`Widget.SetVisibility` (`/Game/Blueprints/New/Blueprints/Player/BP_Player.UI_GameOver` _playerref) "Visible")))

(event `SaveHighscore`
  (bind _gameinstanceref (`self.GameInstanceRef`))
  (bind _savegameref (`/Game/Blueprints/New/Blueprints/BP_GameInstane.SaveGameRef` _gameinstanceref))
  (set `/Game/Blueprints/New/Blueprints/BP_SaveGame.Highscore` (`self.Highscore`) _savegameref)
  (`GameplayStatics.SaveGameToSlot` _savegameref (`/Game/Blueprints/New/Blueprints/BP_GameInstane.SaveGameName` _gameinstanceref)))

(fn `UserConstructionScript`)