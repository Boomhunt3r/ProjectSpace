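; BP_TpBack is a trigger volume that sends cubes back to the storage spot when they enter it.
; On BeginPlay it caches the level's storage, goal and game manager actors.
; An overlapping actor tagged Cube is frozen, rotation-reset, moved to the storage's TP locator and recolored.
; It then asks the game manager to check if the player is still alive, passing the goal's SameColor value.
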(event `self.ReceiveBeginPlay`
  (bind _returnvalue (`GameplayStatics.GetActorOfClass` "/Game/Blueprints/New/Blueprints/BP_Storage.BP_Storage_C"))
  (set `self.Storage Ref` _returnvalue)
  (bind _returnvalue_2 (`GameplayStatics.GetActorOfClass` "/Game/Blueprints/New/Blueprints/Trigger/BP_Goal.BP_Goal_C"))
  (set `self.GoalRef` _returnvalue_2)
  (bind _returnvalue_3 (`GameplayStatics.GetActorOfClass` "/Game/Blueprints/New/Blueprints/Manager/BP_GameManager.BP_GameManager_C"))
  (set `self.GameManagerRef` _returnvalue_3))

(event `self.Box.OnComponentBeginOverlap`
  (params (OverlappedComponent :type "PrimitiveComponent Object Reference") (OtherActor :type "Actor Object Reference") (OtherComp :type "PrimitiveComponent Object Reference") (OtherBodyIndex :type Integer) (bFromSweep :type Boolean) (SweepResult :type "HitResult Structure (by ref)"))
  (if (`self.ActorHasTag` OtherActor "Cube")
    (bind _asbp_cube (cast `/Game/Blueprints/New/Blueprints/Cube/BP_Cube` OtherActor))
    (set `/Game/Blueprints/New/Blueprints/Cube/BP_Cube.CanMove` false _asbp_cube)
    (bind _rootcomponent (`Actor.RootComponent` _asbp_cube))
    (`SceneComponent.K2_SetWorldRotation` :`self` _rootcomponent)
    (`SceneComponent.K2_SetWorldLocation` _rootcomponent (`SceneComponent.K2_GetComponentLocation` (`/Game/Blueprints/New/Blueprints/BP_Storage.TP_Locator` (`self.Storage Ref`))) false false)
    (`/Game/Blueprints/New/Blueprints/Cube/BP_Cube.SetColor` _asbp_cube)
    (`/Game/Blueprints/New/Blueprints/Manager/BP_GameManager.CheckIfAlive` (`self.GameManagerRef`) (`/Game/Blueprints/New/Blueprints/Trigger/BP_Goal.same color` (`self.GoalRef`)))))

(fn `UserConstructionScript`)