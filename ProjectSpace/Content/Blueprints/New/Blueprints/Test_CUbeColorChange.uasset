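; Test actor that repeatedly changes its static mesh's color between blue and yellow with an animated mask transition.
; BeginPlay creates a dynamic material instance, and a FlipFlop picks each NewColor before a timeline animates MaskPosition.
; When the timeline finishes, NewColor is copied to OldColor, the mask resets, and the cycle loops after a delay.
; Tick only runs a Delay, and a random color assignment is left unconnected.
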(event `self.ReceiveBeginPlay`
  (bind _material (`self.Material`))
  (`KismetSystemLibrary.Delay` 1.0)
  (bind _returnvalue (`PrimitiveComponent.CreateDynamicMaterialInstance` (`self.StaticMesh`) 0 "/Game/Blueprints/New/Blueprints/MovingMaterial.MovingMaterial" "None"))
  (set `self.Material` _returnvalue)
  (`/Engine/EditorBlueprintResources/StandardMacros.FlipFlop` :!label _label
    (:`A`
      (`MaterialInstanceDynamic.SetVectorParameterValue` _material "NewColor" (struct :`G` 0.206444 :`B` 1.0 :`A` 1.0))
      (bind _returnvalue_2 (`MaterialInstanceDynamic.K2_GetVectorParameterValue` _material "NewColor"))
      (set `self.New Color` _returnvalue_2))
    (:`B`
      (`MaterialInstanceDynamic.SetVectorParameterValue` _material "NewColor" (struct :`R` 1.0 :`G` 0.959391 :`A` 1.0))
      (bind _returnvalue_3 (`MaterialInstanceDynamic.K2_GetVectorParameterValue` _material "NewColor"))
      (set `self.New Color` _returnvalue_3)))
  (`self.Timeline`))

(event `Timeline`
  (bind _material (`self.Material`))
  (bind (_direction _newtrack_0) (`Timeline|Timeline_0` :!via `PlayFromStart`)
    (:`Update`
      (`MaterialInstanceDynamic.SetScalarParameterValue` (`self.Material`) "MaskPosition" _newtrack_0))
    (:`Finished`
      (`KismetSystemLibrary.Delay` 0.2)
      (`MaterialInstanceDynamic.SetVectorParameterValue` _material "OldColor" (`self.New Color`))
      (`MaterialInstanceDynamic.SetScalarParameterValue` _material "MaskPosition" -2.0)
      (`KismetSystemLibrary.PrintString` "finished")
      (`KismetSystemLibrary.Delay` 3.0)
      (goto _label))))

(event `self.ReceiveTick`
  (params (DeltaSeconds :type "Float (single-precision)"))
  (`KismetSystemLibrary.Delay` 4.0))

(fn `UserConstructionScript`)