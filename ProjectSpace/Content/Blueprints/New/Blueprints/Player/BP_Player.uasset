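; BP_Player is the player Blueprint that sets up the game's UI and relays the start of play.
; On BeginPlay it creates and stores the HUD, main menu and game over widgets, adding all to the viewport but hiding the HUD and game over screen.
; Its StartGame event looks up BP_CubeManager with GetActorOfClass and calls that manager's StartGame.
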(event `self.ReceiveBeginPlay`
  (`|ExecutionSequence`
    (:`then_0`
      (bind _returnvalue (`|CreateWidget` "/Game/Blueprints/New/Blueprints/UI/UI_HUD.UI_HUD_C"))
      (bind _output_get (set `self.UI_HUD` _returnvalue))
      (`UserWidget.AddToViewport` _output_get 0)
      (`Widget.SetVisibility` _output_get "Hidden"))
    (:`then_1`
      (bind _returnvalue_2 (`|CreateWidget` "/Game/Blueprints/New/Blueprints/UI/UI_MainMenu.UI_MainMenu_C"))
      (bind _output_get_2 (set `self.UI_MainMenu` _returnvalue_2))
      (`UserWidget.AddToViewport` _output_get_2 0))
    (:`then_2`
      (bind _returnvalue_3 (`|CreateWidget` "/Game/Blueprints/New/Blueprints/UI/UI_GameOver.UI_GameOver_C"))
      (bind _output_get_3 (set `self.UI_GameOver` _returnvalue_3))
      (`UserWidget.AddToViewport` _output_get_3 0)
      (`Widget.SetVisibility` _output_get_3 "Hidden"))))

(event `Start Game`
  (bind _returnvalue (`GameplayStatics.GetActorOfClass` "/Game/Blueprints/New/Blueprints/Cube/BP_CubeManager.BP_CubeManager_C"))
  (`/Game/Blueprints/New/Blueprints/Cube/BP_CubeManager.Start Game` _returnvalue))

(fn `UserConstructionScript`)