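; Player controller that shows the mouse cursor and detects clicks on actors tagged for painting or erasing.
; On left click it runs a complex Visibility trace under the cursor and checks the hit actor's tags.
; A "Paint" tag prints a blue debug string and an "Erase" tag a green one; no actual paint or erase logic is present.
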(event `self.ReceiveBeginPlay`
  (set `self.bShowMouseCursor` true))

(event `Key|LeftMouseButton`
  (params (Key :type "Key Structure"))
  (bind (_bblockinghit _binitialoverlap _time _distance _location _impactpoint _normal _impactnormal _physmat _hitactor) (`GameplayStatics.BreakHitResult` (`self.GetHitResultUnderCursorByChannel` (`GameplayStatics.GetPlayerController` 0) "TraceTypeQuery1" true)))
  (:`Pressed`
    (if (`self.ActorHasTag` _hitactor "Paint")
      (`KismetSystemLibrary.PrintString` "Hello" true true (struct :`B` 1.0 :`A` 1.0))
      (elif (`self.ActorHasTag` _hitactor "Erase")
        (`KismetSystemLibrary.PrintString` "Hello" true true (struct :`G` 1.0 :`A` 1.0))))))

(fn `UserConstructionScript`)