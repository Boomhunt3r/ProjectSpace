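; BP_Start shifts four board components downward by a fixed step when play begins, apparently as one step of a scrolling or cycling stack.
; BeginPlay stores each board's lowered target, then the ShiftTimer timeline lerps every board from its current position toward it.
; After a Delay fired from the timeline update, Board01 jumps back to the top if its target is the bottom slot; the other boards have no such wrap check.
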(event `self.ReceiveBeginPlay`
  (set `self.Board_01_update` (- (`SceneComponent.RelativeLocation` (`self.Board_01`)) (0.0 0.0 130.0)))
  (set `self.Board_02_Update` (- (`SceneComponent.RelativeLocation` (`self.Board_02`)) (0.0 0.0 130.0)))
  (set `self.Board_03_Update` (- (`SceneComponent.RelativeLocation` (`self.Board_03`)) (0.0 0.0 130.0)))
  (set `self.Board_04_Update` (- (`SceneComponent.RelativeLocation` (`self.Board_04`)) (0.0 0.0 130.0)))
  (bind (_direction _newtrack_0) (`Timeline|Shift Timer`)
    (:`Update`
      (`|ExecutionSequence`
        (:`then_0`
          (`SceneComponent.K2_SetRelativeLocation` (`self.Board_01`) (`KismetMathLibrary.VLerp` (`SceneComponent.RelativeLocation` (`self.Board_01`)) (`self.Board_01_update`) _newtrack_0) false false))
        (:`then_1`
          (`SceneComponent.K2_SetRelativeLocation` (`self.Board_02`) (`KismetMathLibrary.VLerp` (`SceneComponent.RelativeLocation` (`self.Board_02`)) (`self.Board_02_Update`) _newtrack_0) false false))
        (:`then_2`
          (`SceneComponent.K2_SetRelativeLocation` (`self.Board_03`) (`KismetMathLibrary.VLerp` (`SceneComponent.RelativeLocation` (`self.Board_03`)) (`self.Board_03_Update`) _newtrack_0) false false))
        (:`then_3`
          (`SceneComponent.K2_SetRelativeLocation` (`self.Board_04`) (`KismetMathLibrary.VLerp` (`SceneComponent.RelativeLocation` (`self.Board_04`)) (`self.Board_04_Update`) _newtrack_0) false false)
          ;[1 1 1] Check for Teleport
          (`KismetSystemLibrary.Delay` 1.0)
          (if (== (`self.Board_01_update`) (-55.0 0.0 -130.0))
            (`SceneComponent.K2_SetRelativeLocation` (`self.Board_01`) (-55.0 0.0 390.0) false false)))))))

(fn `UserConstructionScript`)