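; Manager Blueprint that runs a rotation of cubes and coordinates the towers that follow them.
; On game start or a next-cube request, it starts the first cube in the list, moves it to the back and sets it as every tower's follow target.
; It also adds to the multiplier on all cubes and disables their movement when the game ends.
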(event `Start Game`
  (`self.StartNextCube`))

(event `StartNextCube`
  (bind _output (`|GetArrayItem` (`self.Cubes`)))
  (if (> (`KismetArrayLibrary.Array_Length` (`self.Cubes`)) 0)
    (set `self.PrevCube` _output)
    (`/Game/Blueprints/New/Blueprints/Cube/BP_Cube.Start Cube` _output)
    (`KismetArrayLibrary.Array_RemoveItem` (`self.Cubes`) (`self.PrevCube`))
    (for _array_element (`self.Towers`)
      (set `/Game/Blueprints/New/Blueprints/Tower/BP_TowerBase.should follow Target` true _array_element)
      (set `/Game/Blueprints/New/Blueprints/Tower/BP_TowerBase.Target Ref` (`self.PrevCube`) _array_element))
    (`KismetArrayLibrary.Array_Add` (`self.Cubes`) (`self.PrevCube`))))

(event `AddToMultplier`
  (params (Multi :type "Float (double-precision)"))
  (for _array_element (`self.Cubes`)
    (set `/Game/Blueprints/New/Blueprints/Cube/BP_Cube.Multiplier` (+ (`/Game/Blueprints/New/Blueprints/Cube/BP_Cube.Multiplier` _array_element) Multi) _array_element)))

(event `EndGame`
  (for _array_element (`self.Cubes`)
    (set `/Game/Blueprints/New/Blueprints/Cube/BP_Cube.CanMove` false _array_element)))

(fn `UserConstructionScript`)